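; BP_Health is a health component for the player in a maze stealth shooter, handling damage, pain and death.
; It binds to the owner's damage event, subtracts clamped damage, plays sounds and broadcasts health and death-count changes through dispatchers.
; At zero health it refills health and has the maze game mode respawn the player.
; A DoOnce gate ignores further hits for two seconds after death.
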(event `self.ReceiveBeginPlay`
  ;[0 0 0] Урон по здоровью игрока, звук боли и смерти, диспатчеры для обновления счётчика здоровья, смертей
  (add `Actor.OnTakeAnyDamage` (`self.GetOwner`) (delegate `Damage`))
  (set `self.Health` (`self.MaxHealth`))
  (bind _asbp_game_mode_maze (cast `/Game/StealthShooter/Blueprints/Core/GameModes/BP_GameModeMaze` (`GameplayStatics.GetGameMode`)))
  (set `self.GameModeMaze` _asbp_game_mode_maze))

(event `Damage`
  (params (DamagedActor :type "Actor Object Reference") (Damage :type "Float (single-precision)") (DamageType :type "DamageType Object Reference") (InstigatedBy :type "Controller Object Reference") (DamageCauser :type "Actor Object Reference"))
  ;[0 0 0] Урон по здоровью игрока, звук боли и смерти, диспатчеры для обновления счётчика здоровья, смертей
  (`/Engine/EditorBlueprintResources/StandardMacros.DoOnce` false :!label _label
    (:`Completed`
      (`|ExecutionSequence`
        (:`then_0`
          (`KismetSystemLibrary.Delay` 0.25)
          (`GameplayStatics.PlaySound2D` (`self.Pain`) 1.0 1.0 0.0 null null))
        (:`then_1`
          (bind _output_get (set `self.Health` (`KismetMathLibrary.FClamp` (- (`self.Health`) Damage) 0.0 (`self.MaxHealth`))))
          (`self.OnChangeHealth` _output_get)
          (if (== _output_get 0.0)
            (`GameplayStatics.PlaySound2D` (`self.Death`) 1.0 1.0 0.0 null null)
            (bind _result (`/Engine/EditorBlueprintResources/StandardMacros.IncrementInt` (`self.Deaths`))
              (:`  `
                (`self.OnChangeLife` _result)
                (set `self.Health` (`self.MaxHealth`))
                (`/Game/StealthShooter/Blueprints/Core/GameModes/BP_GameModeMaze.RebirthPlayer` (`self.GameModeMaze`))
                (`KismetSystemLibrary.Delay` 2.0)
                (`self.OnChangeHealth` (`self.MaxHealth`))
                (goto _label :!via `Reset`)))
            (else
              (goto _label :!via `Reset`))))))))