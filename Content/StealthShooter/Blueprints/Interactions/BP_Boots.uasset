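; BP_Boots is a super boots pickup that spins in the level until the character collects it.
; On box overlap it adds itself to the character's inventory, plays a bonus sound and tags itself Active.
; It then attaches both boot components to the character's foot sockets, sets the Boots flag and closes the Tick gate driving the spin.
; LoadGame reuses this attach path on the player pawn, skipping the pickup steps.
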(event `/Game/StealthShooter/Blueprints/Interface/BPI_SaveGame.LoadGame`
  (bind _mesh (`Character.Mesh` (`self.Character`)))
  ;[0 0 0] Прикрепление суперботинок к персонажу, проигрывание звука, отключение коллизии
  (bind _asbp_character (cast `/Game/StealthShooter/Blueprints/Core/Character/BP_Character` (`GameplayStatics.GetPlayerPawn` 0)))
  (set `self.Character` _asbp_character)
  (`SceneComponent.K2_AttachToComponent` (`self.BootRight`) _mesh "foot_l" "KeepRelative" "KeepRelative" "KeepRelative" true :!label _label)
  (`SceneComponent.K2_AttachToComponent` (`self.BootLeft`) _mesh "foot_r" "KeepRelative" "KeepRelative" "KeepRelative" true)
  (`SceneComponent.K2_SetRelativeTransform` (`self.BootRight`) (`KismetMathLibrary.MakeTransform` (-8.0 9.0 0.0) (struct :`Pitch` 90.0 :`Roll` 180.0) (0.27 0.27 0.27)) false false)
  (`SceneComponent.K2_SetRelativeTransform` (`self.BootLeft`) (`KismetMathLibrary.MakeTransform` (8.0 -3.5 0.0) (struct :`Pitch` -90.0 :`Roll` 180.0) (0.27 0.27 0.27)) false false)
  (set `/Game/StealthShooter/Blueprints/Core/Character/BP_Character.bBoots` true (`self.Character`))
  (goto _label_2 :!via `Close`))

(event `self.ReceiveTick`
  (params (DeltaSeconds :type "Float (single-precision)"))
  ;[0 0 0] Прикрепление суперботинок к персонажу, проигрывание звука, отключение коллизии
  (`/Engine/EditorBlueprintResources/StandardMacros.Gate` false :!label _label_2
    (:`Exit`
      (`self.K2_AddActorLocalRotation` (`KismetMathLibrary.MakeRotator` 0.0 0.0 (* DeltaSeconds 360.0))))))

(event `self.Box.OnComponentBeginOverlap`
  (params (OverlappedComponent :type "PrimitiveComponent Object Reference") (OtherActor :type "Actor Object Reference") (OtherComp :type "PrimitiveComponent Object Reference") (OtherBodyIndex :type Integer) (bFromSweep :type Boolean) (SweepResult :type "HitResult Structure (by ref)"))
  ;[0 0 0] Прикрепление суперботинок к персонажу, проигрывание звука, отключение коллизии
  (bind _asbp_character (cast `/Game/StealthShooter/Blueprints/Core/Character/BP_Character` OtherActor))
  (bind _output_get (set `self.Character` _asbp_character))
  (`/Game/StealthShooter/Blueprints/Core/Character/BP_Character.ChangeInventory` _output_get true self (`self.Texture`))
  (`GameplayStatics.PlaySound2D` "/Game/StealthShooter/Assets/Sound/A_Bonus.A_Bonus" 1.0 1.0 0.0 null null)
  (`KismetArrayLibrary.Array_Add` (`self.Tags`) "Active")
  (goto _label))

(fn `UserConstructionScript`)