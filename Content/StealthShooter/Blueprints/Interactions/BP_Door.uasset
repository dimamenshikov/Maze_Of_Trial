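; BP_Door is a color-locked swinging door that opens on interaction when the nearby player's Keys contain its Color.
; A dot product picks the swing direction away from the player, and a timeline lerps the door's yaw.
; Leaving the trigger box reverses the timeline to close it, with a 2D sound played during motion.
; The construction script tints frame and door with that Color through dynamic materials.
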(event `self.ReceiveBeginPlay`
  ;[0 0 0] Сохранение ссылки на игрока, создание звука
  (bind _asbp_character (cast `/Game/StealthShooter/Blueprints/Core/Character/BP_Character` (`GameplayStatics.GetPlayerPawn` 0)))
  (set `self.Character` _asbp_character)
  (bind _returnvalue (`GameplayStatics.CreateSound2D` "/Game/StealthShooter/Assets/Sound/A_OpenCloseDoor.A_OpenCloseDoor" 1.0 1.0 0.0 null))
  (set `self.SoundDoor` _returnvalue))

(event `/Game/StealthShooter/Blueprints/Interface/BPI_Interaction.Interaction`
  (params (On :type Boolean))
  (bind _sounddoor (`self.SoundDoor`))
  (bind (_relativerotation_roll _relativerotation_pitch _relativerotation_yaw) (`KismetMathLibrary.BreakRotator` (`SceneComponent.RelativeRotation` (`self.Door`))))
  ;[0 0 0] Открывание в сторону противоположной направлению движения персонажа, проигрывание звука, закрывание двери
  (if (and (`self.bPlayerNear`) (!= (`KismetArrayLibrary.Array_Find` (`/Game/StealthShooter/Blueprints/Core/Character/BP_Character.Keys` (`self.Character`)) (`self.Color`)) -1))
    (set `self.StartAngle` _relativerotation_yaw)
    (set `self.EndAngle` (`KismetMathLibrary.SelectFloat` 90.0 -90.0 (< (`KismetMathLibrary.Dot_VectorVector` (- (`self.K2_GetActorLocation` (`self.Character`)) (`self.K2_GetActorLocation`)) (`self.GetActorForwardVector`)) 0.0)))
    (`AudioComponent.Play` _sounddoor 4.5)
    (`AudioComponent.SetPaused` _sounddoor false)
    (bind (_direction _angle) (`Timeline|OpenCloseDoor` :!label _label)
      (:`Update`
        (`SceneComponent.K2_SetRelativeRotation` (`self.Door`) (`KismetMathLibrary.MakeRotator` 0.0 0.0 (`KismetMathLibrary.Lerp` (`self.StartAngle`) (`self.EndAngle`) _angle)) false false))
      (:`Finished`
        (`AudioComponent.SetPaused` (`self.SoundDoor`) true)))))

(event `self.Box.OnComponentEndOverlap`
  (params (OverlappedComponent :type "PrimitiveComponent Object Reference") (OtherActor :type "Actor Object Reference") (OtherComp :type "PrimitiveComponent Object Reference") (OtherBodyIndex :type Integer))
  (bind _sounddoor (`self.SoundDoor`))
  (bind (_relativerotation_roll _relativerotation_pitch _relativerotation_yaw) (`KismetMathLibrary.BreakRotator` (`SceneComponent.RelativeRotation` (`self.Door`))))
  ;[0 0 0] Открывание в сторону противоположной направлению движения персонажа, проигрывание звука, закрывание двери
  (if (`self.ActorHasTag` OtherActor "Player")
    (set `self.bPlayerNear` false)
    (set `self.EndAngle` _relativerotation_yaw)
    (set `self.StartAngle` 0.0)
    (`AudioComponent.Play` _sounddoor 8.0)
    (`AudioComponent.SetPaused` _sounddoor false)
    (goto _label :!via `Reverse`)))

(event `self.Box.OnComponentBeginOverlap`
  (params (OverlappedComponent :type "PrimitiveComponent Object Reference") (OtherActor :type "Actor Object Reference") (OtherComp :type "PrimitiveComponent Object Reference") (OtherBodyIndex :type Integer) (bFromSweep :type Boolean) (SweepResult :type "HitResult Structure (by ref)"))
  ;[0 0 0] Открывание в сторону противоположной направлению движения персонажа, проигрывание звука, закрывание двери
  (if (`self.ActorHasTag` OtherActor "Player")
    (set `self.bPlayerNear` true)))

(fn `UserConstructionScript`
  (bind _color (`self.Color`))
  ;[0 0 0] Создание динамического материала и установка заданного цвета
  (bind _returnvalue (`PrimitiveComponent.CreateDynamicMaterialInstance` (`self.Frame`) 0 null "None"))
  (`MaterialInstanceDynamic.SetVectorParameterValue` _returnvalue "Color" _color)
  (bind _returnvalue_2 (`PrimitiveComponent.CreateDynamicMaterialInstance` (`self.Door`) 0 null "None"))
  (`MaterialInstanceDynamic.SetVectorParameterValue` _returnvalue_2 "Color" _color))