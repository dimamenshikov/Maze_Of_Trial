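; Laser turret that tracks the player and deals continuous damage, with damage per second set by the game instance's difficulty at BeginPlay.
; Activate raises or lowers an activation counter; while positive, a next-tick loop rotates the gun toward the player, with the frame following yaw only.
; Once aimed, it applies damage, stretches the beam by Z scale and starts the laser sound, resetting beam and sound when the counter reaches zero.
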(event `self.ReceiveBeginPlay`
  ;[0 0 0] Создание звука, установка урона в зависимости от сложности
  (bind _returnvalue (`GameplayStatics.CreateSound2D` "/Game/StealthShooter/Assets/Sound/A_Laser.A_Laser" 1.0 1.0 0.0 null))
  (set `self.laser` _returnvalue)
  (bind _asbp_game_instance_maze (cast `/Game/StealthShooter/Blueprints/Core/BP_GameInstanceMaze` (`GameplayStatics.GetGameInstance`)))
  (set `self.Damage` (select `/Game/StealthShooter/Blueprints/Enums/E_Difficulty` (`/Game/StealthShooter/Blueprints/Core/BP_GameInstanceMaze.Difficulty` _asbp_game_instance_maze) :`NewEnumerator0` 80.0 :`NewEnumerator1` 50.0 :`NewEnumerator2` 30.0)))

(event `/Game/StealthShooter/Blueprints/Interface/BPI_Interaction.Activate`
  (params (Activate :type Boolean))
  (bind _turrel (`self.Turrel`))
  (bind _turrel_2 (`self.Turrel`))
  (bind _laser (`self.laser`))
  (bind _returnvalue (`SceneComponent.K2_GetComponentRotation` _turrel))
  (bind (_returnvalue_roll _returnvalue_pitch _returnvalue_yaw) (`KismetMathLibrary.BreakRotator` (`SceneComponent.K2_GetComponentRotation` _turrel_2)))
  (bind _returnvalue_2 (`KismetMathLibrary.FindLookAtRotation` (`SceneComponent.K2_GetComponentLocation` _turrel) (+ (`self.K2_GetActorLocation` (`GameplayStatics.GetPlayerPawn` 0)) (0.0 0.0 35.0))))
  (bind (_returnvalue_roll_2 _returnvalue_pitch_2 _returnvalue_yaw_2) (`KismetMathLibrary.BreakRotator` (`KismetMathLibrary.RInterpTo_Constant` _returnvalue _returnvalue_2 (`GameplayStatics.GetWorldDeltaSeconds`) 150.0)))
  ;[0 0 0] Поворот на персонажа, нанесение урона
  (bind _output_get (set `self.CountActivate` (`KismetMathLibrary.Max` (+ (`self.CountActivate`) (`KismetMathLibrary.SelectInt` 1 -1 Activate)))))
  (if (> _output_get 0) :!label _label
    (`SceneComponent.K2_SetWorldRotation` _turrel_2 (`KismetMathLibrary.MakeRotator` 0.0 _returnvalue_pitch_2 _returnvalue_yaw_2) false false)
    (`SceneComponent.K2_SetWorldRotation` (`self.TurrelFrame`) (`KismetMathLibrary.MakeRotator` 0.0 0.0 _returnvalue_yaw) false false)
    (if (== _returnvalue _returnvalue_2 :`ErrorTolerance` 0.5)
      (`GameplayStatics.ApplyDamage` (`GameplayStatics.GetPlayerPawn` 0) (* (`GameplayStatics.GetWorldDeltaSeconds`) (`self.Damage`)))
      (`SceneComponent.SetRelativeScale3D` (`self.Scene`) (`KismetMathLibrary.MakeVector` 1.0 1.0 (/ (`KismetMathLibrary.VSize` (- (`SceneComponent.K2_GetComponentLocation` (`self.Scene`)) (`self.K2_GetActorLocation` (`GameplayStatics.GetPlayerPawn` 0)) (0.0 0.0 -35.0))) 5.0)))
      (`|ExecutionSequence`
        (:`then_0`
          (`/Engine/EditorBlueprintResources/StandardMacros.DoOnce` false :!label _label_2
            (:`Completed`
              (`AudioComponent.SetPaused` _laser false)
              (`AudioComponent.Play` _laser 0.0))))
        (:`then_1`
          (`KismetSystemLibrary.DelayUntilNextTick` :!label _label_3)
          (goto _label)))
      (else
        (goto _label_3)))
    (else
      (`SceneComponent.SetRelativeScale3D` (`self.Scene`) (1.0 1.0 1.0))
      (`AudioComponent.SetPaused` (`self.laser`) true)
      (goto _label_2 :!via `Reset`))))

(fn `UserConstructionScript`)