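; BP_TriggerBox is a trigger volume that activates the actors inside it when the player enters and deactivates them on exit.
; On BeginPlay, a debug-drawn multi box trace matching the volume caches the hit actors in OverlappingActors.
; Overlaps by actors tagged Player send each cached actor an Activate message with true or false.
; The construction script sizes the box from BoxSize and raises it so the origin sits at its base.
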(event `self.ReceiveBeginPlay`
  (bind (_boxextent_x _boxextent_y _boxextent_z) (`KismetMathLibrary.BreakVector` (`BoxComponent.BoxExtent` (`self.Box`))))
  (bind _returnvalue (+ (`self.K2_GetActorLocation`) (`KismetMathLibrary.MakeVector` 0.0 0.0 _boxextent_z)))
  ;[0 0 0] Сохранение всех акторов внутри коллизии
  (bind _outhits (`KismetSystemLibrary.BoxTraceMulti` :`Start` _returnvalue :`End` _returnvalue :`HalfSize` (`KismetMathLibrary.MakeVector` _boxextent_x _boxextent_y _boxextent_z) :`TraceChannel` "TraceTypeQuery3" :`DrawDebugType` "ForDuration"))
  (for _array_element _outhits
    (`KismetArrayLibrary.Array_Add` (`self.Overlapping Actors`) (`.HitActor` (`GameplayStatics.BreakHitResult` _array_element)))))

(event `self.Box.OnComponentBeginOverlap`
  (params (OverlappedComponent :type "PrimitiveComponent Object Reference") (OtherActor :type "Actor Object Reference") (OtherComp :type "PrimitiveComponent Object Reference") (OtherBodyIndex :type Integer) (bFromSweep :type Boolean) (SweepResult :type "HitResult Structure (by ref)"))
  ;[0 0 0] Включение всех акторов в коллизии при входе игрока в коллизию
  (if (`self.ActorHasTag` OtherActor "Player")
    (for _array_element (`self.Overlapping Actors`)
      (message `/Game/StealthShooter/Blueprints/Interface/BPI_Interaction.Activate` _array_element true))))

(event `self.Box.OnComponentEndOverlap`
  (params (OverlappedComponent :type "PrimitiveComponent Object Reference") (OtherActor :type "Actor Object Reference") (OtherComp :type "PrimitiveComponent Object Reference") (OtherBodyIndex :type Integer))
  ;[0 0 0] Отключение всех акторов в коллизии при выходе игрока из коллизии
  (if (`self.ActorHasTag` OtherActor "Player")
    (for _array_element (`self.Overlapping Actors`)
      (message `/Game/StealthShooter/Blueprints/Interface/BPI_Interaction.Activate` _array_element false))))

(fn `UserConstructionScript`
  (bind _box (`self.Box`))
  (bind (_boxsize_x _boxsize_y _boxsize_z) (`KismetMathLibrary.BreakVector` (`self.BoxSize`)))
  ;[0 0 0] Настройка размеров коллизии
  (`BoxComponent.SetBoxExtent` _box (`KismetMathLibrary.MakeVector` _boxsize_x _boxsize_y _boxsize_z) true)
  (`SceneComponent.K2_SetRelativeLocation` _box (`KismetMathLibrary.MakeVector` 0.0 0.0 _boxsize_z) false false))