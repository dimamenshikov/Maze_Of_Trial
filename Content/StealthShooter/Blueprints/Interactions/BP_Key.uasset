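; BP_Key is a colored key pickup that spins in the level and goes into the player's inventory on touch.
; The construction script tints a dynamic material with the key's Color, and Activate starts or stops the Rotate timeline driving the spin.
; Overlap with BP_Character adds the color and inventory entry, plays a sound, tags the key "Active", then hides and disables it.
; LoadGame reuses that same hide-and-disable path.
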(event `/Game/StealthShooter/Blueprints/Interface/BPI_Interaction.Activate`
  (params (Activate :type Boolean))
  ;[0 0 0] Сокрытия ключа, отключение коллизии, добавка ключа в инвентарь при подборе персонажем, вращение ключа
  (if Activate
    (`Timeline|Rotate` :!label _label
      (:`Update`
        (`self.K2_AddActorLocalRotation` (`KismetMathLibrary.MakeRotator` 0.0 0.0 (* (`GameplayStatics.GetWorldDeltaSeconds`) 360.0)))))
    (else
      (goto _label :!via `Stop`))))

(event `/Game/StealthShooter/Blueprints/Interface/BPI_SaveGame.LoadGame`
  ;[0 0 0] Сокрытия ключа, отключение коллизии, добавка ключа в инвентарь при подборе персонажем, вращение ключа
  (`self.SetActorHiddenInGame` true :!label _label_2)
  (`self.SetActorEnableCollision` false)
  (goto _label :!via `Stop`))

(event `self.Box.OnComponentBeginOverlap`
  (params (OverlappedComponent :type "PrimitiveComponent Object Reference") (OtherActor :type "Actor Object Reference") (OtherComp :type "PrimitiveComponent Object Reference") (OtherBodyIndex :type Integer) (bFromSweep :type Boolean) (SweepResult :type "HitResult Structure (by ref)"))
  ;[0 0 0] Сокрытия ключа, отключение коллизии, добавка ключа в инвентарь при подборе персонажем, вращение ключа
  (bind _asbp_character (cast `/Game/StealthShooter/Blueprints/Core/Character/BP_Character` OtherActor))
  (bind _output_get (set `self.Character` _asbp_character))
  (`KismetArrayLibrary.Array_Add` (`/Game/StealthShooter/Blueprints/Core/Character/BP_Character.Keys` _output_get) (`self.Color`))
  (`/Game/StealthShooter/Blueprints/Core/Character/BP_Character.ChangeInventory` (`self.Character`) true self (`self.Texture`))
  (`GameplayStatics.PlaySound2D` "/Game/StealthShooter/Assets/Sound/A_Key.A_Key" 1.0 1.0 0.0 null null)
  (`KismetArrayLibrary.Array_Add` (`self.Tags`) "Active")
  (goto _label_2))

(fn `UserConstructionScript`
  (bind _returnvalue (`PrimitiveComponent.CreateDynamicMaterialInstance` (`self.Key`) 0 null "None"))
  (`MaterialInstanceDynamic.SetVectorParameterValue` _returnvalue "Color" (`self.Color`)))