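; BP_Gate is an interactable gate that opens and closes on an Activate event by shrinking its Z scale to zero and back.
; A timeline paced by Time drives the scale, while a 2D gate sound plays until the movement finishes.
; Opening adds an "Active" tag; closing waits for Duration, then removes it and reverses the timeline.
; LoadGame replays the opening with the sound muted, restoring volume when finished.
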(event `self.ReceiveBeginPlay`
  (bind (_returnvalue_x _returnvalue_y _returnvalue_z) (`KismetMathLibrary.BreakVector` (`self.GetActorScale3D`)))
  ;[0 0 0] Установка скорости открывания ворот, создание звука
  (set `self.ScaleZ` _returnvalue_z)
  (`TimelineComponent.SetPlayRate` (`self.UpDown`) (/ 1.0 (`self.Time`)))
  (bind _returnvalue (`GameplayStatics.CreateSound2D` "/Game/StealthShooter/Assets/Sound/A_Gate.A_Gate" 1.0 1.0 0.0 null false false))
  (set `self.GateSound` _returnvalue))

(event `/Game/StealthShooter/Blueprints/Interface/BPI_Interaction.Activate`
  (params (Activate :type Boolean))
  (bind (_returnvalue_x _returnvalue_y) (`KismetMathLibrary.BreakVector` (`self.GetActorScale3D`)))
  (bind _tags (`self.Tags`))
  ;[0 0 0] Поднимание и опускание ворот при нажатии на кнопку
  (if Activate
    (`KismetArrayLibrary.Array_Add` _tags "Active")
    (bind _gatesound (`self.GateSound`)
      (:`then`
        (`AudioComponent.SetPaused` _gatesound false)
        (`AudioComponent.Play` _gatesound 0.0)
        (bind (_direction _scalez) (`Timeline|UpDown` :!label _label)
          (:`Update`
            (`self.SetActorScale3D` (`KismetMathLibrary.MakeVector` _returnvalue_x _returnvalue_y (`KismetMathLibrary.Lerp` (`self.ScaleZ`) 0.0 _scalez))))
          (:`Finished`
            (bind _gatesound_2 (`self.GateSound`)
              (:`then`
                (`AudioComponent.SetPaused` _gatesound_2 true)
                (`AudioComponent.SetVolumeMultiplier` _gatesound_2 1.0))
              (:`else`)))))
      (:`else`
        (goto _label)))
    (else
      (`KismetSystemLibrary.Delay` (`self.Duration`))
      (`KismetArrayLibrary.Array_RemoveItem` _tags "Active")
      (bind _gatesound_3 (`self.GateSound`)
        (:`then`
          (`AudioComponent.SetPaused` _gatesound_3 false)
          (`AudioComponent.Play` _gatesound_3 0.0)
          (goto _label :!via `Reverse`))
        (:`else`
          (goto _label :!via `Reverse`))))))

(event `/Game/StealthShooter/Blueprints/Interface/BPI_SaveGame.LoadGame`
  ;[0 0 0] Активация при загрузке уровня
  (bind _gatesound (`self.GateSound`)
    (:`then`
      (`AudioComponent.SetVolumeMultiplier` _gatesound 0.0))
    (:`else`
      _))
  (`/Game/StealthShooter/Blueprints/Interface/BPI_Interaction.Activate` true))

(fn `UserConstructionScript`)