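; BP_Treasure is a maze pickup that completes the current mission when the character overlaps it.
; On overlap it plays a sound, adds itself to the character's inventory, tags itself "Active" and shows timed mission messages ending with the maze-escape objective.
; It also immediately sets the character's Treasure flag, disables collision and hides.
; LoadGame reuses that final step on the player pawn, skipping sound, inventory and messages.
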(event `self.Treasure.OnComponentBeginOverlap`
  (params (OverlappedComponent :type "PrimitiveComponent Object Reference") (OtherActor :type "Actor Object Reference") (OtherComp :type "PrimitiveComponent Object Reference") (OtherBodyIndex :type Integer) (bFromSweep :type Boolean) (SweepResult :type "HitResult Structure (by ref)"))
  ;[0 0 0] Добавление сокровища в инвентарь, показ миссий, отключение коллизий, сокрытие актора
  (bind _asbp_character (cast `/Game/StealthShooter/Blueprints/Core/Character/BP_Character` OtherActor))
  (set `self.Character` _asbp_character)
  (`GameplayStatics.PlaySound2D` "/Game/StealthShooter/Assets/Sound/A_Bonus.A_Bonus" 1.0 1.0 0.0 null null)
  (`/Game/StealthShooter/Blueprints/Core/Character/BP_Character.ChangeInventory` (`self.Character`) true self (`self.Texture`))
  (`KismetArrayLibrary.Array_Add` (`self.Tags`) "Active")
  (`|ExecutionSequence`
    (:`then_0`
      (bind _asbp_game_mode_maze (cast `/Game/StealthShooter/Blueprints/Core/GameModes/BP_GameModeMaze` (`GameplayStatics.GetGameMode`)))
      (bind _interface (`/Game/StealthShooter/Blueprints/Core/GameModes/BP_GameModeMaze.Interface` _asbp_game_mode_maze))
      (`/Game/StealthShooter/Widgets/WBP_Interface.ShowMissionText` _interface "Миссия выполнена!" (make `SlateColor` (struct :`G` 1.0)))
      (`KismetSystemLibrary.Delay` 4.1)
      (`/Game/StealthShooter/Widgets/WBP_Interface.ShowMissionText` _interface "Новая миссия!" (make `SlateColor` (struct :`R` 1.0 :`G` 1.0)))
      (`KismetSystemLibrary.Delay` 4.1)
      (`/Game/StealthShooter/Widgets/WBP_Interface.ShowMissionText` _interface "Выбраться из лабиринта" (make `SlateColor` (struct :`R` 1.0 :`G` 1.0 :`B` 1.0))))
    (:`then_1`
      (set `/Game/StealthShooter/Blueprints/Core/Character/BP_Character.bTreasure` true (`self.Character`) :!label _label)
      (`self.SetActorEnableCollision` false)
      (`self.SetActorHiddenInGame` true))))

(event `/Game/StealthShooter/Blueprints/Interface/BPI_SaveGame.LoadGame`
  ;[0 0 0] Добавление сокровища в инвентарь, показ миссий, отключение коллизий, сокрытие актора
  (bind _asbp_character (cast `/Game/StealthShooter/Blueprints/Core/Character/BP_Character` (`GameplayStatics.GetPlayerPawn` 0)))
  (set `self.Character` _asbp_character)
  (goto _label))

(fn `UserConstructionScript`)