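; BP_Lever is an interactable lever that activates a linked list of actors.
; Interaction, debounced by a half-second DoOnce, runs a timeline that pitches the handle, with a switch sound on forward throws.
; When the timeline finishes, a second DoOnce, re-armed on each interaction, messages every linked actor once.
; AutoUp makes the handle return by itself; otherwise a FlipFlop alternates its direction per interaction.
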(event `/Game/StealthShooter/Blueprints/Interface/BPI_Interaction.Interaction`
  (params (On :type Boolean))
  ;[0 0 0] Поднятие/Опускание рычага, активация акторов, которыми управляет рычаг
  (`/Engine/EditorBlueprintResources/StandardMacros.DoOnce` false :!label _label
    (:`Completed`
      (`|ExecutionSequence`
        (:`then_0`
          (`KismetSystemLibrary.Delay` 0.5)
          (goto _label :!via `Reset`))
        (:`then_1`
          (goto _label_4 :!via `Reset`))
        (:`then_2`
          (if (`self.bAutoUp`)
            (`GameplayStatics.PlaySound2D` "/Game/StealthShooter/Assets/Sound/A_LeverSwitch.A_LeverSwitch" 1.0 1.0 0.0 null null :!label _label_2)
            (bind (_direction _angle) (`Timeline|UpDownLever` :!label _label_3)
              (:`Update`
                (`SceneComponent.K2_SetRelativeRotation` (`self.Switch handle`) (`KismetMathLibrary.MakeRotator` 0.0 _angle) false false))
              (:`Finished`
                (`/Engine/EditorBlueprintResources/StandardMacros.DoOnce` false :!label _label_4
                  (:`Completed`
                    (for _array_element (`self.Actors`)
                      (message `/Game/StealthShooter/Blueprints/Interface/BPI_Interaction.Activate` _array_element (`self.bActivateActor`)))
                    (if (`self.bAutoUp`)
                      (goto _label_3 :!via `Reverse`))))))
            (else
              (`/Engine/EditorBlueprintResources/StandardMacros.FlipFlop`
                (:`A`
                  (goto _label_2))
                (:`B`
                  (goto _label_3 :!via `Reverse`))))))))))

(fn `UserConstructionScript`)