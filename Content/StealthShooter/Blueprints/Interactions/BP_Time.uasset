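; BP_Time is a clock pickup that adds five minutes to the maze game mode's time when the player collects it.
; Tick spins the actor around yaw one full turn per second through a Gate that starts open.
; Overlap of the Clock component by a Player-tagged actor updates BP_GameModeMaze's Time and plays a bonus sound.
; The pickup then hides, disables collision and closes the Gate to stop spinning, rather than being destroyed.
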(event `self.ReceiveTick`
  (params (DeltaSeconds :type "Float (single-precision)"))
  ;[0 0 0] Вращение часов, добавление 5 минут при подборе их игроком
  (`/Engine/EditorBlueprintResources/StandardMacros.Gate` false :!label _label
    (:`Exit`
      (`self.K2_AddActorLocalRotation` (`KismetMathLibrary.MakeRotator` 0.0 0.0 (* DeltaSeconds 360.0))))))

(event `self.Clock.OnComponentBeginOverlap`
  (params (OverlappedComponent :type "PrimitiveComponent Object Reference") (OtherActor :type "Actor Object Reference") (OtherComp :type "PrimitiveComponent Object Reference") (OtherBodyIndex :type Integer) (bFromSweep :type Boolean) (SweepResult :type "HitResult Structure (by ref)"))
  (bind _asbp_game_mode_maze (cast `/Game/StealthShooter/Blueprints/Core/GameModes/BP_GameModeMaze` (`GameplayStatics.GetGameMode`) :!pure true))
  ;[0 0 0] Вращение часов, добавление 5 минут при подборе их игроком
  (if (`self.ActorHasTag` OtherActor "Player")
    (set `/Game/StealthShooter/Blueprints/Core/GameModes/BP_GameModeMaze.Time` (+ (`/Game/StealthShooter/Blueprints/Core/GameModes/BP_GameModeMaze.Time` _asbp_game_mode_maze) 300.0) _asbp_game_mode_maze)
    (`GameplayStatics.PlaySound2D` "/Game/StealthShooter/Assets/Sound/A_Bonus.A_Bonus" 1.0 1.0 0.0 null null)
    (`self.SetActorHiddenInGame` true)
    (`self.SetActorEnableCollision` false)
    (goto _label :!via `Close`)))

(fn `UserConstructionScript`)