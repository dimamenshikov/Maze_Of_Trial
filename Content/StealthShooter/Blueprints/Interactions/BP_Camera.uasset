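; Security camera for the stealth shooter that sweeps a yaw patrol on a timeline and raises the alarm on spotting the player.
; A Beam overlap confirmed by a visibility trace starts the warning sound, activates the linked turret and turns the camera to track the player.
; Losing sight or leaving TriggerZone silences both and eases the camera back to patrol.
; Tracking and return run as gated next-tick loops instead of Event Tick.
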(event `/Game/StealthShooter/Blueprints/Interface/BPI_Interaction.Activate`
  (params (Activate :type Boolean))
  (bind _tags (`self.Tags`))
  ;[0 0 0] Запуск или остановка патрулирования
  (if Activate
    (`KismetArrayLibrary.Array_Add` _tags "Active")
    (set `self.bPatrol` true)
    (bind (_direction _rotate) (`Timeline|RotatePatrol` :!label _label)
      (:`Update`
        (bind _output_get (set `self.Rotate` _rotate))
        (if (`self.bPatrol`)
          (`SceneComponent.K2_SetRelativeRotation` (`self.Camera`) (`KismetMathLibrary.MakeRotator` 0.0 (`self.Relative Rotation`) _output_get) false false))))
    (else
      (`KismetArrayLibrary.Array_RemoveItem` _tags "Active")
      (goto _label :!via `Stop`))))

(event `/Game/StealthShooter/Blueprints/Interface/BPI_SaveGame.LoadGame`
  ;[0 0 0] Запуск патрулирования при загрузке уровня
  (`self.Patrol` true))

(event `self.ReceiveBeginPlay`
  (bind (_relativerotation_roll _relativerotation_pitch) (`KismetMathLibrary.BreakRotator` (`SceneComponent.RelativeRotation` (`self.Camera`))))
  ;[0 0 0] Сохранение нужных ссылок в переменные, создание звука
  (set `self.Relative Rotation` _relativerotation_pitch)
  (bind _returnvalue (`GameplayStatics.CreateSound2D` "/Game/StealthShooter/Assets/Sound/A_Warning.A_Warning" 1.0 1.0 0.0 null false false))
  (set `self.Warning` _returnvalue)
  (bind _asbp_game_mode_maze (cast `/Game/StealthShooter/Blueprints/Core/GameModes/BP_GameModeMaze` (`GameplayStatics.GetGameMode`)))
  (set `self.GameModeMaze` _asbp_game_mode_maze)
  (bind _asbp_character (cast `/Game/StealthShooter/Blueprints/Core/Character/BP_Character` (`GameplayStatics.GetPlayerPawn` 0)))
  (set `self.Character` _asbp_character))

(event `Shoot`
  (params (Shoot :type Boolean))
  (bind _camera (`self.Camera`))
  (bind _camera_2 (`self.Camera`))
  ;[0 0 0] Активирование пушки, проигрывание звука при входе игрока в коллизию актора
  (if Shoot
    (`|ExecutionSequence`
      (:`then_0`
        (goto _label_2 :!via `Open`))
      (:`then_1`
        (`/Engine/EditorBlueprintResources/StandardMacros.Gate` false :!label _label_2
          (:`Exit`
            (`SceneComponent.K2_SetWorldRotation` _camera (`KismetMathLibrary.RInterpTo_Constant` (`SceneComponent.K2_GetComponentRotation` _camera_2) (`KismetMathLibrary.FindLookAtRotation` (`SceneComponent.K2_GetComponentLocation` _camera_2) (`self.K2_GetActorLocation` (`GameplayStatics.GetPlayerPawn` 0))) (`GameplayStatics.GetWorldDeltaSeconds`) 120.0) false false)
            (bind _outhit (`KismetSystemLibrary.LineTraceSingle` (`SceneComponent.K2_GetComponentLocation` _camera) (`self.K2_GetActorLocation` (`GameplayStatics.GetPlayerPawn` 0)) "TraceTypeQuery1"))
            (cast `/Game/StealthShooter/Blueprints/Core/Character/BP_Character` (`.HitActor` (`GameplayStatics.BreakHitResult` _outhit))
              (:`then`
                (`KismetSystemLibrary.DelayUntilNextTick`)
                (goto _label_2))
              (:`CastFailed`
                (`|ExecutionSequence`
                  (:`then_0`
                    (goto _label_3 :!via `Reset`))
                  (:`then_1`
                    (bind _warning (`self.Warning`)
                      (:`then`
                        (`AudioComponent.SetPaused` _warning true))
                      (:`else`
                        _))
                    (`self.Shoot` false)
                    (`self.Patrol` true)
                    (if (`self.bChangeActiveTurrel`)
                      (message `/Game/StealthShooter/Blueprints/Interface/BPI_Interaction.Activate` (`self.Turrel`) false)
                      (set `self.bChangeActiveTurrel` false))))))))))
    (else
      (goto _label_2 :!via `Close`))))

(event `self.Beam.OnComponentBeginOverlap`
  (params (OverlappedComponent :type "PrimitiveComponent Object Reference") (OtherActor :type "Actor Object Reference") (OtherComp :type "PrimitiveComponent Object Reference") (OtherBodyIndex :type Integer) (bFromSweep :type Boolean) (SweepResult :type "HitResult Structure (by ref)"))
  ;[0 0 0] Активирование пушки, проигрывание звука при входе игрока в коллизию актора
  (bind _outhit (`KismetSystemLibrary.LineTraceSingle` (`SceneComponent.K2_GetComponentLocation` (`self.Camera`)) (`self.K2_GetActorLocation` (`GameplayStatics.GetPlayerPawn` 0)) "TraceTypeQuery1"))
  (if (`self.ActorHasTag` OtherActor "Player")
    (cast `/Game/StealthShooter/Blueprints/Core/Character/BP_Character` (`.HitActor` (`GameplayStatics.BreakHitResult` _outhit)))
    (`/Engine/EditorBlueprintResources/StandardMacros.DoOnce` true :!label _label_3
      (:`Completed`
        (bind _warning (`self.Warning`)
          (:`then`
            (`AudioComponent.SetPaused` _warning false)
            (`AudioComponent.Play` _warning 0.0))
          (:`else`
            _))
        (`|ExecutionSequence`
          (:`then_0`
            (`self.Patrol` false))
          (:`then_1`
            (`self.Shoot` true)
            (message `/Game/StealthShooter/Blueprints/Interface/BPI_Interaction.Activate` (`self.Turrel`) true)
            (set `self.bChangeActiveTurrel` true)))))))

(event `self.TriggerZone.OnComponentBeginOverlap`
  (params (OverlappedComponent :type "PrimitiveComponent Object Reference") (OtherActor :type "Actor Object Reference") (OtherComp :type "PrimitiveComponent Object Reference") (OtherBodyIndex :type Integer) (bFromSweep :type Boolean) (SweepResult :type "HitResult Structure (by ref)"))
  ;[0 0 0] Активирование пушки, проигрывание звука при входе игрока в коллизию актора
  (if (`self.ActorHasTag` OtherActor "Player")
    (`/Engine/EditorBlueprintResources/StandardMacros.DoOnce` false :!label _label_4
      (:`Completed`
        (`|ExecutionSequence`
          (:`then_0`
            (goto _label_3 :!via `Reset`))
          (:`then_1`
            (goto _label_5 :!via `Reset`)))))))

(event `self.TriggerZone.OnComponentEndOverlap`
  (params (OverlappedComponent :type "PrimitiveComponent Object Reference") (OtherActor :type "Actor Object Reference") (OtherComp :type "PrimitiveComponent Object Reference") (OtherBodyIndex :type Integer))
  ;[0 0 0] Активирование пушки, проигрывание звука при входе игрока в коллизию актора
  (if (`self.ActorHasTag` OtherActor "Player")
    (`/Engine/EditorBlueprintResources/StandardMacros.DoOnce` true :!label _label_5
      (:`Completed`
        (bind _warning (`self.Warning`)
          (:`then`
            (`AudioComponent.SetPaused` _warning true))
          (:`else`
            _))
        (`self.Shoot` false)
        (if (`self.bChangeActiveTurrel`)
          (message `/Game/StealthShooter/Blueprints/Interface/BPI_Interaction.Activate` (`self.Turrel`) false)
          (set `self.bChangeActiveTurrel` false))
        (`|ExecutionSequence`
          (:`then_0`
            (`self.Patrol` true))
          (:`then_1`
            (goto _label_4 :!via `Reset`)))))))

(event `Patrol`
  (params (Patrol :type Boolean))
  (bind _relative_rotation (`self.Relative Rotation`))
  (bind _rotate (`self.Rotate`))
  (bind _relativerotation (`SceneComponent.RelativeRotation` (`self.Camera`)))
  ;[0 0 0] Возвращение к позиции патрулирования
  (set `self.bPatrol` false)
  (if Patrol
    (`|ExecutionSequence`
      (:`then_0`
        (goto _label_6 :!via `Open`))
      (:`then_1`
        (`/Engine/EditorBlueprintResources/StandardMacros.Gate` false :!label _label_6
          (:`Exit`
            (`SceneComponent.K2_SetRelativeRotation` (`self.Camera`) (`KismetMathLibrary.RInterpTo_Constant` _relativerotation (`KismetMathLibrary.MakeRotator` 0.0 _relative_rotation _rotate) (`GameplayStatics.GetWorldDeltaSeconds`) 60.0) false false)
            (if (== _relativerotation (`KismetMathLibrary.MakeRotator` 0.0 _relative_rotation _rotate) :`ErrorTolerance` 0.05)
              (set `self.bPatrol` true)
              (else
                (`KismetSystemLibrary.DelayUntilNextTick`)
                (goto _label_6)))))))
    (else
      (goto _label_6 :!via `Close`))))

(fn `UserConstructionScript`)