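; BP_Projectile is a cannon puzzle projectile that damages the player on contact.
; On BeginPlay it turns once toward the player character, spawns smoke and sets its damage from the difficulty stored in BP_GameInstanceMaze.
; Any overlap with its Box spawns an explosion and destroys it, applying damage only to actors tagged Player.
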(event `self.ReceiveBeginPlay`
  ;[0 0 0] Запись ссылок на нужные объекты, запись сложности, поворот на персонажа, проигрывание эффекта выстрела
  (bind _asbp_character (cast `/Game/StealthShooter/Blueprints/Core/Character/BP_Character` (`GameplayStatics.GetPlayerPawn` 0)))
  (set `self.Character` _asbp_character)
  (`self.K2_SetActorRotation` (`KismetMathLibrary.FindLookAtRotation` (`self.K2_GetActorLocation`) (`self.K2_GetActorLocation` (`self.Character`))))
  (`GameplayStatics.SpawnEmitterAtLocation` "/Game/StealthShooter/Assets/Effects/Smoke/PS_Smoke.PS_Smoke" (`self.K2_GetActorLocation`))
  (bind _asbp_game_instance_maze (cast `/Game/StealthShooter/Blueprints/Core/BP_GameInstanceMaze` (`GameplayStatics.GetGameInstance`)))
  (set `self.Damage` (select `/Game/StealthShooter/Blueprints/Enums/E_Difficulty` (`/Game/StealthShooter/Blueprints/Core/BP_GameInstanceMaze.Difficulty` _asbp_game_instance_maze) :`NewEnumerator0` 15.0 :`NewEnumerator1` 10.0 :`NewEnumerator2` 5.0)))

(event `self.Box.OnComponentBeginOverlap`
  (params (OverlappedComponent :type "PrimitiveComponent Object Reference") (OtherActor :type "Actor Object Reference") (OtherComp :type "PrimitiveComponent Object Reference") (OtherBodyIndex :type Integer) (bFromSweep :type Boolean) (SweepResult :type "HitResult Structure (by ref)"))
  ;[0 0 0] Столкновение, нанесение урона персонажу, включение звука, эффекта, ичтожение снаряда
  (if (`self.ActorHasTag` OtherActor "Player")
    (`GameplayStatics.ApplyDamage` OtherActor (`self.Damage`) null self))
  (`GameplayStatics.SpawnEmitterAtLocation` "/Game/StealthShooter/Assets/Effects/Explosion/PS_Explosion.PS_Explosion" (`self.K2_GetActorLocation`))
  (`self.K2_DestroyActor`))

(fn `UserConstructionScript`)