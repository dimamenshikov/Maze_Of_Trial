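; BP_Cannon is a puzzle turret that, while activated, repeatedly fires physics projectiles aimed to intercept the player.
; It samples player velocity over one frame, then solves a quartic (moving) or quadratic (stationary) equation for the shortest flight time, retrying after recharge if none exists.
; The ballistic launch velocity includes a quarter-second lead that covers the frame-stepped barrel turn, paced by FPS measured at BeginPlay.
; Each shot plays a recoil timeline and restarts the cycle.
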(event Custom|Launch
  (bind _staticmesh (Variables|Default|GetStaticMesh))
  (bind _staticmesh_2 (Variables|Default|GetStaticMesh))
  (bind _calculateprojectilevelocity (Variables|Default|GetCalculateProjectileVelocity))
  (bind _actor (Variables|StartValue|GetActor))
  (bind _fps (Variables|StartValue|GetFPS))
  (bind _returnvalue (Transformation|GetWorldRotation _staticmesh_2))
  (bind _returnvalue_2 (Transformation|GetWorldRotation _staticmesh))
  (bind _returnvalue_3 (/ _fps 4))
  (bind _returnvalue_4 (+ _actor _calculateprojectilevelocity))
  (bind _returnvalue_5 (Math|Rotator|FindRelativeLookatRotation (Math|Transform|MakeTransform _actor _returnvalue "1.000000,1.000000,1.000000") _returnvalue_4))
  ;[0 0 0] Ручной поворот пушки и запуск снаряда
  (Variables|RotateCannon|SetPitch (.pitch _returnvalue_5))
  (Variables|RotateCannon|SetYaw (.yaw _returnvalue_5))
  (if (and (< (Math|Float|Absolute(Float) (Variables|RotateCannon|GetYaw)) 0.01) (< (Math|Float|Absolute(Float) (Variables|RotateCannon|GetPitch)) 0.01))
    (Utilities|FlowControl|Delay 0.2167)
    (else
      (Transformation|SetWorldRotation (Variables|Default|GetStaticMesh) (Math|Rotator|MakeRotator 0.0 (+ (/ (Variables|RotateCannon|GetPitch) _returnvalue_3) (.pitch _returnvalue_2)) (+ (/ (Variables|RotateCannon|GetYaw) _returnvalue_3) (.yaw _returnvalue_2))) false false :!label _label)
      (Math|Integer|IncrementInt (Variables|RotateCannon|GetAccout)
        (:%20%20
          (Utilities|FlowControl|DelayUntilNextTick)
          (if (== (Variables|RotateCannon|GetAccout) (/ (Variables|StartValue|GetFPS) 4))
            (Variables|RotateCannon|SetAccout 0)
            (else
              (goto _label)))))))
  (bind _returnvalue_6 (Game|SpawnActorfromClass "/Game/StealthShooter/Blueprints/Puzzle/Cannon/BP_Projectile.BP_Projectile_C" (Math|Transform|MakeTransform (Variables|StartValue|GetActor) "0, 0, 0" "0.500000,0.500000,0.500000") "Undefined" "MultiplyWithRoot" 0 0))
  (Audio|PlaySound2D "/Game/StealthShooter/Assets/Sound/A_Burst.A_Burst" 1.0 1.0 0.0 0 0)
  (Physics|SetPhysicsLinearVelocity (Variables|/Game/StealthShooter/Blueprints/Puzzle/Cannon/BP_Projectile.BP_Projectile_C|GetBox _returnvalue_6) (Variables|Default|GetCalculateProjectileVelocity) false "None")
  (Class|PrimitiveComponent|SetPhysicsAngularVelocityinDegrees (Variables|/Game/StealthShooter/Blueprints/Puzzle/Cannon/BP_Projectile.BP_Projectile_C|GetBox _returnvalue_6) (Math|Vector|MakeVector 0.0 0.0 1e+03) false "None")
  (CallFunction|Restart (- (Variables|StartValue|GetRecharge) 0.25))
  (bind _alpha (Timeline|CannonOffset PlayFromStart)
    (:Update
      (Transformation|SetRelativeLocation (Variables|Default|GetStaticMesh) (Math|Vector|Lerp(Vector) (Variables|StartValue|GetStartCannonOffset) (* (Math|Vector|GetForwardVector (Variables|Default|GetStaticMesh)) -5e+01) _alpha) false false))))

(event Custom|Restart
  (params (Recharge :type Float%20%28double-precision%29))
  ;[0 0 0] Начало расчёта, подготовка необходимых зачений для расчётов
  ;;[0 0 0] Перезарядка
  (Utilities|FlowControl|Delay Recharge)
  (CallFunction|StartCalculate))

(event Custom|CalculateVelocity
  (bind _playervelocity (Variables|StartValue|GetPlayerVelocity))
  (bind _timeprojectile (Variables|Default|GetTimeProjectile))
  (bind _deltalocation (Variables|StartValue|GetDeltaLocation))
  (bind _timeprojectile_2 (Variables|Default|GetTimeProjectile))
  (bind _returnvalue (+ _timeprojectile_2 0.25))
  (bind _returnvalue_2 (* _returnvalue _playervelocity))
  (bind _returnvalue_3 (+ _returnvalue_2 _deltalocation))
  (bind _returnvalue_4 (/ _returnvalue_3 _timeprojectile))
  ;[0 0 0] Расчёт скорости снаряда
  (Variables|Default|SetCalculateProjectileVelocity (Math|Vector|MakeVector (.x _returnvalue_4) (.y _returnvalue_4) (- (.z _returnvalue_4) (* _timeprojectile (Variables|StartValue|GetG) 0.5))))
  (CallFunction|Launch))

(event Custom|StartCalculate
  (bind _character (Variables|StartValue|GetCharacter))
  (bind _returnvalue (Transformation|GetActorLocation _character))
  ;[0 0 0] Начало расчёта, подготовка необходимых зачений для расчётов
  (Utilities|FlowControl|Gate true
    (:Exit
      (bind _output_get (Variables|StartValue|SetPlayer _returnvalue))
      (Utilities|FlowControl|DelayUntilNextTick)
      (Variables|StartValue|SetPlayerVelocity (* (- _returnvalue _output_get) (Variables|StartValue|GetFPS)))
      (bind _output_get_2 (Variables|StartValue|SetPlayer (Transformation|GetActorLocation (Variables|StartValue|GetCharacter))))
      (bind _output_get_3 (Variables|StartValue|SetDeltaLocation (- _output_get_2 (Variables|StartValue|GetActor))))
      (Variables|SplitVector|SetDx (.x _output_get_3))
      (Variables|SplitVector|SetDy (.y _output_get_3))
      (Variables|SplitVector|SetDz (.z _output_get_3))
      (Variables|SplitVector|SetPVz (.z (Variables|StartValue|GetPlayerVelocity)))
      (Variables|SplitVector|SetPVy (.y (Variables|StartValue|GetPlayerVelocity)))
      (Variables|SplitVector|SetPVx (.x (Variables|StartValue|GetPlayerVelocity)))
      ;[0 0 0] Расчёт времени полёта снаряда в зависимости от типа движения игрока (движение в плоскости, нет движения)
      (if (Utilities|Operators|NotEqual(!=) :A (Variables|StartValue|GetPlayerVelocity) :ErrorTolerance 0.0001)
        (bind (_exist _roots) (CallFunction|EducationFourthDegree (Variables|StartValue|GetCoefficient_G) (|(0-({969759DA-460E-A0F2-0307-D5BE5832FA12}*{F3DB24D1-47F0-56B9-C163-D993B3CC21F5}))) (|((((VectorLengthSquared({DF99E89C-451D-B747-583A-599798A31F4D}))-({B22EB0EA-40C2-CFD9-4685-A393976D1437}*{F3DB24D1-47F0-56B9-C163-D993B3CC21F5}))-(Power({81370CEB-4F51-0F22-553F-628FC78D48A2},2)))-((0.250000*{969759DA-460E-A0F2-0307-D5BE5832FA12})*{F3DB24D1-47F0-56B9-C163-D993B3CC21F5}))) (|((VectorLengthSquared({DF99E89C-451D-B747-583A-599798A31F4D}))+(2*((({DD4468FB-47EB-7EF1-3279-5DB459122FE6}*{2FCD02A0-4119-D942-9EE3-3DB0BCCDA968})+({09404DE4-4333-E9A0-5B4D-7A92D06745F2}*{2E5E7BFD-4708-A1E2-CDAF-F7A94FAF6583}))+({969759DA-460E-A0F2-0307-D5BE5832FA12}*{B22EB0EA-40C2-CFD9-4685-A393976D1437}))))) (|(((Power(((0.250000*{DD4468FB-47EB-7EF1-3279-5DB459122FE6})+{2FCD02A0-4119-D942-9EE3-3DB0BCCDA968}),2))+(Power(((0.250000*{09404DE4-4333-E9A0-5B4D-7A92D06745F2})+{2E5E7BFD-4708-A1E2-CDAF-F7A94FAF6583}),2)))+(Power(((0.250000*{969759DA-460E-A0F2-0307-D5BE5832FA12})+{B22EB0EA-40C2-CFD9-4685-A393976D1437}),2))))))
        (Utilities|CalculateTime _exist _roots
          (:True
            (CallFunction|CalculateVelocity)))
        (else
          (bind (_exist_2 _roots_2) (CallFunction|EducationSecondDegree (Variables|StartValue|GetCoefficient_G) (|(0-(({F3DB24D1-47F0-56B9-C163-D993B3CC21F5}*{B22EB0EA-40C2-CFD9-4685-A393976D1437})+(Power({81370CEB-4F51-0F22-553F-628FC78D48A2},2))))) (|(VectorLengthSquared({9326EE84-419D-A722-EAEE-A581967CC4B9})))))
          (bind _time (Utilities|CalculateTime _exist_2 _roots_2)
            (:True
              (Variables|Default|SetTimeProjectile (Math|Float|Sqrt _time))
              (Variables|StartValue|SetPlayerVelocity "0, 0, 0")
              (CallFunction|CalculateVelocity))))))))

(event EventBeginPlay
  ;[0 0 0] Начало расчёта, подготовка необходимых зачений для расчётов
  (bind _asbp_character (Utilities|Casting|CastToBP_Character (Game|Player|GetPlayerPawn 0)))
  (Variables|StartValue|SetCharacter _asbp_character)
  (Variables|StartValue|SetActor (Transformation|GetActorLocation))
  (Utilities|FlowControl|DelayUntilNextTick)
  (Variables|StartValue|SetFPS (Math|Float|Truncate (/ 1.0 (Utilities|Time|GetWorldDeltaSeconds))))
  (Variables|StartValue|SetCoefficient_G (|((power({F3DB24D1-47F0-56B9-C163-D993B3CC21F5},2))/4))))

(event EventActivate
  (params (Activate :type Boolean))
  (bind _character (Variables|StartValue|GetCharacter))
  (bind _returnvalue (Transformation|GetActorLocation _character))
  ;[0 0 0] Начало расчёта, подготовка необходимых зачений для расчётов
  (if Activate
    (Utilities|FlowControl|Sequence
      (:then_0
        (Utilities|FlowControl|Gate true) ; enters at Open
      )
      (:then_1
        (CallFunction|StartCalculate)))
    (else
      (Utilities|FlowControl|Gate true) ; enters at Close
    )))

(fn ConstructionScript)