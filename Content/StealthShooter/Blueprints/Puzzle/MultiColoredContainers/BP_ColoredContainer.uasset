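; Carryable cube for the colored-container puzzle that the player picks up and drops through the Interaction event.
; A FlipFlop alternates between attaching it in front of the character with collision off and detaching it with collision and physics on.
; Pickup only happens when the character has no attached actors, though the FlipFlop toggles regardless.
; The construction script stores a dynamic material instance of the cube.
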(event `self.ReceiveBeginPlay`
  ;[0 0 0] Сохранение ссылки на персонажа
  (bind _asbp_character (cast `/Game/StealthShooter/Blueprints/Core/Character/BP_Character` (`GameplayStatics.GetPlayerPawn` 0)))
  (set `self.Character` _asbp_character))

(event `/Game/StealthShooter/Blueprints/Interface/BPI_Interaction.Interaction`
  (params (On :type Boolean))
  (bind _cube (`self.Cube`))
  ;[0 0 0] Прикрепление и открепление куба к персонажу
  (`/Engine/EditorBlueprintResources/StandardMacros.FlipFlop`
    (:`A`
      (if (`KismetArrayLibrary.Array_IsEmpty` (`self.GetAttachedActors` (`self.Character`) true true))
        (`self.K2_AttachToActor` (`self.Character`) "None" "KeepWorld" "KeepWorld" "KeepWorld")
        (`PrimitiveComponent.SetCollisionEnabled` (`self.Cube`) "NoCollision")
        (`self.K2_SetActorRelativeLocation` (80.0 0.0 20.0))))
    (:`B`
      (`self.K2_DetachFromActor` "KeepWorld" "KeepWorld" "KeepWorld")
      (`PrimitiveComponent.SetCollisionEnabled` _cube "QueryAndPhysics")
      (`PrimitiveComponent.SetSimulatePhysics` _cube true))))

(fn `UserConstructionScript`
  ;[0 0 0] Создание динамического материала
  (bind _returnvalue (`PrimitiveComponent.CreateDynamicMaterialInstance` (`self.Cube`) 0 null "None"))
  (set `self.Material` _returnvalue))