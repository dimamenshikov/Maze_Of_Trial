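; Controller for the colored-container puzzle that spawns up to 16 randomly colored BP_ColoredContainer actors at its own location.
; On BeginPlay it builds the color pool by duplicating each of PipeControl's StartColors.
; Each delayed Activate passes a Gate set by Open, spawns one container and tints it with a color drawn without replacement, closing the Gate at the limit.
; Destroy removes all containers and resets the counter and color pool.
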(event `self.ReceiveBeginPlay`
  ;[0 0 0] Создание массива цветов на 16 кубов
  (for _array_element (`/Game/StealthShooter/Blueprints/Puzzle/MultiColoredContainers/BP_WireSystem.StartColors` (`self.PipeControl`))
    (for _ (range 2)
      (`KismetArrayLibrary.Array_Add` (`self.StartColors`) _array_element)))
  (set `self.Colors` (`self.StartColors`)))

(event `/Game/StealthShooter/Blueprints/Interface/BPI_Interaction.Activate`
  (params (Activate :type Boolean))
  (bind _colors (`self.Colors`))
  ;[0 0 0] Создание кубов и присвоение ему случайного цвета
  (`KismetSystemLibrary.Delay` 0.25)
  (`/Engine/EditorBlueprintResources/StandardMacros.Gate` true :!label _label
    (:`Exit`
      (bind _output_get (set `self.RandomIndex` (`.OutIndex` (`KismetArrayLibrary.Array_Random` (`self.Colors`)))))
      (set `self.RandomColor` (`|GetArrayItem` _colors _output_get))
      (`KismetArrayLibrary.Array_Remove` _colors (`self.RandomIndex`))
      (bind _returnvalue (`|SpawnActorFromClass` "/Game/StealthShooter/Blueprints/Puzzle/MultiColoredContainers/BP_ColoredContainer.BP_ColoredContainer_C" (`KismetMathLibrary.MakeTransform` (`self.K2_GetActorLocation`)) "Undefined" "MultiplyWithRoot" null null))
      (`KismetArrayLibrary.Array_Add` (`self.Containers`) _returnvalue)
      (`MaterialInstanceDynamic.SetVectorParameterValue` (`/Game/StealthShooter/Blueprints/Puzzle/MultiColoredContainers/BP_ColoredContainer.Material` _returnvalue) "Color" (`self.RandomColor`))
      (bind _result (`/Engine/EditorBlueprintResources/StandardMacros.IncrementInt` (`self.Index`))
        (:`  `
          (if (> _result 15)
            (goto _label :!via `Close`)))))))

(event `Open`
  (params (Open :type Boolean))
  ;[0 0 0] Создание кубов и присвоение ему случайного цвета
  (if Open
    (goto _label :!via `Open`)
    (else
      (goto _label :!via `Close`))))

(event `Destroy`
  ;[0 0 0] Уничтожение всех кубов
  (for _array_element (`self.Containers`)
    (`/Engine/EditorBlueprintResources/StandardMacros.IsValid` _array_element
      (:`Is Valid`
        (`self.K2_DestroyActor` _array_element))))
  (`KismetArrayLibrary.Array_Clear` (`self.Containers`))
  (set `self.Index` 0)
  (set `self.Colors` (`self.StartColors`)))

(fn `UserConstructionScript`)