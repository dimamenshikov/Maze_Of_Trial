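; Puzzle pipe that accepts colored containers and reports whether their color matches its own cap material.
; Start runs one timeline forward or in reverse twice, toggling between Z-scale and rotation phases via FlipFlop, with crane audio and cap visibility changes.
; Box overlap destroys the container and fires the OnColoredContainer dispatcher with color, pipe and match result.
; A DoOnce gate resets immediately on a match, after a delay otherwise.
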(event `self.ReceiveBeginPlay`
  ;[0 0 0] Сокрытие трубы и создание звука
  (`self.SetActorScale3D` (1.0 1.0 0.0))
  (bind _returnvalue (`GameplayStatics.CreateSound2D` "/Game/StealthShooter/Assets/Sound/A_Crane.A_Crane" 1.0 1.0 0.0 null))
  (set `self.SoundPipe` _returnvalue))

(event `Start`
  (params (Start :type Boolean))
  (bind _soundpipe (`self.SoundPipe`))
  ;[0 0 0] Поднимание и опускание труб
  (`SceneComponent.SetHiddenInGame` (`self.Cap`) false false)
  (`AudioComponent.SetPaused` _soundpipe false)
  (`AudioComponent.Play` _soundpipe 4.1)
  (if Start :!label _label
    (bind (_direction _alpha) (`Timeline|UpDownPipe` :!via `PlayFromStart` :!label _label_2)
      (:`Update`
        (if (`self.bRotate`)
          (`SceneComponent.K2_SetRelativeRotation` (`self.Scene`) (`KismetMathLibrary.MakeRotator` (* _alpha 270.0)) false false)
          (else
            (`self.SetActorScale3D` (`KismetMathLibrary.MakeVector` 1.0 1.0 _alpha)))))
      (:`Finished`
        (`/Engine/EditorBlueprintResources/StandardMacros.FlipFlop`
          (:`A`
            (set `self.bRotate` (not (`self.bRotate`)))
            (`AudioComponent.SetPaused` (`self.SoundPipe`) true)
            (goto _label))
          (:`B`
            (`SceneComponent.SetHiddenInGame` (`self.Cap`) true false)))))
    (else
      (goto _label_2 :!via `ReverseFromEnd`))))

(event `self.Box.OnComponentBeginOverlap`
  (params (OverlappedComponent :type "PrimitiveComponent Object Reference") (OtherActor :type "Actor Object Reference") (OtherComp :type "PrimitiveComponent Object Reference") (OtherBodyIndex :type Integer) (bFromSweep :type Boolean) (SweepResult :type "HitResult Structure (by ref)"))
  ;[0 0 0] Вызов диспатчера при попадании куба в трубу
  (`/Engine/EditorBlueprintResources/StandardMacros.IsValid` OtherActor :!label _label_3
    (:`Is Valid`
      (bind _asbp_colored_container (cast `/Game/StealthShooter/Blueprints/Puzzle/MultiColoredContainers/BP_ColoredContainer` OtherActor))
      (`/Engine/EditorBlueprintResources/StandardMacros.DoOnce` false :!label _label_4
        (:`Completed`
          (bind _returnvalue (`MaterialInstanceDynamic.K2_GetVectorParameterValue` (`/Game/StealthShooter/Blueprints/Puzzle/MultiColoredContainers/BP_ColoredContainer.Material` _asbp_colored_container) "Color"))
          (`self.K2_DestroyActor` _asbp_colored_container)
          (bind _returnvalue_2 (`MaterialInstanceDynamic.K2_GetVectorParameterValue` (`self.Material`) "Color"))
          (bind _returnvalue_3 (== _returnvalue_2 _returnvalue))
          (`self.OnColoredContainer` _returnvalue self _returnvalue_3)
          (if _returnvalue_3
            (goto _label_4 :!via `Reset`)
            (else
              (`KismetSystemLibrary.Delay` 6.0)
              (`|ExecutionSequence`
                (:`then_0`
                  (goto _label_4 :!via `Reset`))
                (:`then_1`
                  (goto _label_3))))))))))

(fn `UserConstructionScript`
  ;[0 0 0] Создание динамического материала крышки
  (bind _returnvalue (`PrimitiveComponent.CreateDynamicMaterialInstance` (`self.Cap`) 0 null "None"))
  (set `self.Material` _returnvalue))