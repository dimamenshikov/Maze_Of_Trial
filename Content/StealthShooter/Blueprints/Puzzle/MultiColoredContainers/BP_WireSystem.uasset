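; Puzzle controller for colored pipes and containers, showing progress as growing wires built in the construction script.
; Activate alternately raises pipes with unique random colors mirrored on their wires, then opens ContainerControl, or lowers and resets everything, with DoOnce gates blocking overlap.
; SetColorWire extends a pipe's wire on a color match or spawns a temporary segment that falls off on mismatch.
; Two matches per pipe in total activate the linked actors.
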(event `self.ReceiveBeginPlay`
  ;[0 0 0] Сохранение всех труб в массив и подписка на диспатчер когда в трубу попадает куб
  (bind _outactors (`GameplayStatics.GetAllActorsOfClass` "/Game/StealthShooter/Blueprints/Puzzle/MultiColoredContainers/BP_Pipe.BP_Pipe_C"))
  (bind _output_get (set `self.StartPipes` _outactors))
  (set `self.Quantity` (`KismetArrayLibrary.Array_Length` _output_get))
  (bind _output_get_2 (set `self.Pipes` _output_get))
  (for _array_element _output_get_2
    (add `/Game/StealthShooter/Blueprints/Puzzle/MultiColoredContainers/BP_Pipe.OnColoredContainer` _array_element (`|CreateDelegate` :!event `SetColorWire`))))

(event `/Game/StealthShooter/Blueprints/Interface/BPI_Interaction.Activate`
  (params (Activate :type Boolean))
  (bind _randompipe (`self.RandomPipe`))
  (bind _randomcolor (`self.RandomColor`))
  (bind _containercontrol (`self.ContainerControl`))
  ;[0 0 0] Вызов поднятия и опускания у всех труб присвоение им случайного цвета
  (`/Engine/EditorBlueprintResources/StandardMacros.FlipFlop`
    (:`A`
      (set `self.Count` 0)
      (`/Engine/EditorBlueprintResources/StandardMacros.DoOnce` false :!label _label
        (:`Completed`
          (if (> (`self.Quantity`) (`self.Index`)) :!label _label_2
            (bind _output_get (set `self.RandomPipe` (`KismetArrayLibrary.Array_Random` (`self.Pipes`))))
            (`/Game/StealthShooter/Blueprints/Puzzle/MultiColoredContainers/BP_Pipe.Start` _output_get true)
            (bind _output_get_2 (set `self.RandomColor` (`KismetArrayLibrary.Array_Random` (`self.Colors`))))
            (`MaterialInstanceDynamic.SetVectorParameterValue` (`/Game/StealthShooter/Blueprints/Puzzle/MultiColoredContainers/BP_Pipe.Material` _randompipe) "Color" _output_get_2)
            (`MaterialInstanceDynamic.SetVectorParameterValue` (`|GetArrayItem` (`self.Materials`) (`KismetArrayLibrary.Array_Find` (`self.StartPipes`) _randompipe)) "Color" _randomcolor)
            (`KismetArrayLibrary.Array_RemoveItem` (`self.Colors`) _randomcolor)
            (`KismetArrayLibrary.Array_RemoveItem` (`self.Pipes`) (`self.RandomPipe`))
            (`/Engine/EditorBlueprintResources/StandardMacros.IncrementInt` (`self.Index`)
              (:`  `
                (`KismetSystemLibrary.Delay` 1.5)
                (goto _label_2)))
            (else
              (`KismetSystemLibrary.Delay` 5.0)
              (`/Game/StealthShooter/Blueprints/Puzzle/MultiColoredContainers/BP_ContainerControl.Open` (`self.ContainerControl`) true)
              (goto _label_3 :!via `Reset`))))))
    (:`B`
      (`/Engine/EditorBlueprintResources/StandardMacros.DoOnce` true :!label _label_3
        (:`Completed`
          (for _array_element (`self.StartPipes`)
            (`/Game/StealthShooter/Blueprints/Puzzle/MultiColoredContainers/BP_Pipe.Start` _array_element false))
          (`|ExecutionSequence`
            (:`then_0`
              (`KismetSystemLibrary.Delay` 6.6)
              (goto _label :!via `Reset`))
            (:`then_1`
              (`self.Reset`)
              (set `self.Pipes` (`self.StartPipes`))
              (set `self.Colors` (`self.StartColors`))
              (set `self.Index` 0)
              (`/Game/StealthShooter/Blueprints/Puzzle/MultiColoredContainers/BP_ContainerControl.Destroy` _containercontrol)
              (`KismetSystemLibrary.Delay` 6.5)
              (`/Game/StealthShooter/Blueprints/Puzzle/MultiColoredContainers/BP_ContainerControl.Open` _containercontrol false))))))))

(event `SetColorWire`
  (params (Color :type "LinearColor Structure") (PIpe :type "/Game/StealthShooter/Blueprints/Puzzle/MultiColoredContainers/BP_Pipe Object Reference") (Coincidence :type Boolean))
  (bind _wiress (`self.Wiress`))
  (bind _returnvalue (`KismetArrayLibrary.Array_Find` (`self.StartPipes`) PIpe))
  (bind _output (`|GetArrayItem` _wiress _returnvalue))
  (bind (_relativelocation_x _relativelocation_y _relativelocation_z) (`KismetMathLibrary.BreakVector` (`SceneComponent.RelativeLocation` _output)))
  (bind (_relativescale3d_x _relativescale3d_y _relativescale3d_z) (`KismetMathLibrary.BreakVector` (`SceneComponent.RelativeScale3D` _output)))
  ;[0 0 0] Вызов удлинения провода или создание нового провода при несовпадении цвета трубы и цвета куба
  (if Coincidence
    (`self.Offset` (`|GetArrayItem` _wiress _returnvalue))
    (bind _result (`/Engine/EditorBlueprintResources/StandardMacros.IncrementInt` (`self.Count`))
      (:`  `
        (if (== _result (* 2 (`self.Quantity`)))
          (`KismetSystemLibrary.Delay` 1.5)
          (`GameplayStatics.PlaySound2D` "/Game/StealthShooter/Assets/Sound/A_Button.A_Button" 1.0 1.0 0.0 null null)
          (for _array_element (`self.Actor`)
            (message `/Game/StealthShooter/Blueprints/Interface/BPI_Interaction.Activate` _array_element true)))))
    (else
      (bind _returnvalue_2 (`AddComponent|NODE_AddSceneComponent-1` :`RelativeTransform` (`KismetMathLibrary.MakeTransform` (`KismetMathLibrary.MakeVector` 0.0 (* _relativescale3d_z -100.0) _relativelocation_z) (struct :`Roll` -90.0) (1.0 1.0 0.0))))
      (bind _returnvalue_3 (`AddComponent|NODE_AddStaticMeshComponent-1` :`RelativeTransform` (`KismetMathLibrary.MakeTransform` (0.0 0.0 50.0) (struct) (0.5 0.5 1.0))))
      (`SceneComponent.K2_AttachToComponent` _returnvalue_3 _returnvalue_2 "None" "KeepRelative" "KeepRelative" "KeepRelative" true)
      (bind _returnvalue_4 (`PrimitiveComponent.CreateDynamicMaterialInstance` _returnvalue_3 0 null "None"))
      (`MaterialInstanceDynamic.SetVectorParameterValue` _returnvalue_4 "Color" Color)
      (`self.Offset` _returnvalue_2)
      (`KismetSystemLibrary.Delay` 2.0)
      (`PrimitiveComponent.SetSimulatePhysics` _returnvalue_3 true)
      (`KismetSystemLibrary.Delay` 3.0)
      (`ActorComponent.K2_DestroyComponent` _returnvalue_2)
      (`ActorComponent.K2_DestroyComponent` _returnvalue_3))))

(event `Reset`
  ;[0 0 0] Возвращение всех проводов
  (bind (_direction _alpha) (`Timeline|ResetAllWire` :!via `PlayFromStart`)
    (:`Update`
      (for _array_element (`self.Wiress`)
        (bind (_relativescale3d_x _relativescale3d_y _relativescale3d_z) (`KismetMathLibrary.BreakVector` (`SceneComponent.RelativeScale3D` _array_element)))
        (`SceneComponent.SetRelativeScale3D` _array_element (`KismetMathLibrary.MakeVector` 1.0 1.0 (`KismetMathLibrary.Lerp` _relativescale3d_z 0.0 _alpha)))))))

(event `Offset`
  (params (Wire :type "SceneComponent Object Reference"))
  (bind _relative_scale_3d_z (`self.Relative Scale 3D Z`))
  (bind (_relativescale3d_x _relativescale3d_y _relativescale3d_z) (`KismetMathLibrary.BreakVector` (`SceneComponent.RelativeScale3D` Wire)))
  ;[0 0 0] Удлинение провода
  (set `self.Relative Scale 3D Z` _relativescale3d_z)
  (bind (_direction _alpha) (`Timeline|OffsetWire` :!via `PlayFromStart`)
    (:`Update`
      (`SceneComponent.SetRelativeScale3D` Wire (`KismetMathLibrary.MakeVector` 1.0 1.0 (`KismetMathLibrary.Lerp` _relative_scale_3d_z (+ _relative_scale_3d_z 3.0) _alpha))))))

(fn `UserConstructionScript`
  ;[0 0 0] Создание 8 проводов
  (for _index (range 8)
    (bind _returnvalue (`AddComponent|NODE_AddSceneComponent-0` :`RelativeTransform` (`KismetMathLibrary.MakeTransform` (`KismetMathLibrary.MakeVector` 0.0 0.0 (`KismetMathLibrary.Conv_IntToDouble` (* _index 100))) (struct :`Roll` -90.0) (1.0 1.0 0.0))))
    (bind _returnvalue_2 (`AddComponent|NODE_AddStaticMeshComponent-0` :`RelativeTransform` (`KismetMathLibrary.MakeTransform` (0.0 0.0 50.0) (struct) (0.5 0.5 1.0))))
    (`SceneComponent.K2_AttachToComponent` _returnvalue_2 _returnvalue "None" "KeepRelative" "KeepRelative" "KeepRelative" true)
    (bind _returnvalue_3 (`PrimitiveComponent.CreateDynamicMaterialInstance` _returnvalue_2 0 null "None"))
    (`KismetArrayLibrary.Array_Add` (`self.Materials`) _returnvalue_3)
    (`KismetArrayLibrary.Array_Add` (`self.Wiress`) _returnvalue)))