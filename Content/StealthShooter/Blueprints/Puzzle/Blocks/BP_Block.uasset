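; BP_Block is a puzzle cube that the nearby player interacts with to roll it one step away from them.
; FindRotate snaps the player's relative direction to a quarter turn, and CheckObstacle box-traces the opposite side for blockers.
; A timeline animates the tip and move, then restores orientation and plays an impact sound, with DoOnce preventing overlapping rolls.
; The GameModeMaze rebirth event returns the block to its start location.
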(event `self.ReceiveBeginPlay`
  (bind (_returnvalue_roll _returnvalue_pitch _returnvalue_yaw) (`KismetMathLibrary.BreakRotator` (`self.K2_GetActorRotation`)))
  ;[0 0 0] Сохранение нужных ссылок в переменные, возвращение на начальную позицию при смерти персонажа
  (`|ExecutionSequence`
    (:`then_0`
      (bind _asbp_character (cast `/Game/StealthShooter/Blueprints/Core/Character/BP_Character` (`GameplayStatics.GetPlayerPawn` 0)))
      (set `self.Character` _asbp_character))
    (:`then_1`
      (set `self.StartRotationYaw` (mod _returnvalue_yaw 90.0))
      (set `self.StartLocation` (`self.K2_GetActorLocation`)))
    (:`then_2`
      (bind _asbp_game_mode_maze (cast `/Game/StealthShooter/Blueprints/Core/GameModes/BP_GameModeMaze` (`GameplayStatics.GetGameMode`)))
      (add `/Game/StealthShooter/Blueprints/Core/GameModes/BP_GameModeMaze.OnRebirthPlayer` _asbp_game_mode_maze (delegate `Reset`)))))

(event `Reset`
  ;[0 0 0] Сохранение нужных ссылок в переменные, возвращение на начальную позицию при смерти персонажа
  (`self.K2_SetActorLocation` (`self.StartLocation`)))

(event `/Game/StealthShooter/Blueprints/Interface/BPI_Interaction.Interaction`
  (params (On :type Boolean))
  (bind (_previousrotate_roll _previousrotate_pitch) (`KismetMathLibrary.BreakRotator` (`self.PreviousRotate`)))
  (bind (_previousrotate_roll_2 _previousrotate_pitch_2 _previousrotate_yaw) (`KismetMathLibrary.BreakRotator` (`self.PreviousRotate`)))
  ;[0 0 0] Поворот куба
  (`/Engine/EditorBlueprintResources/StandardMacros.DoOnce` false :!label _label
    (:`Completed`
      (if (and (not (`self.CheckObstacle` (`self.Find Rotate`))) (< (`KismetMathLibrary.VSize` (- (`self.K2_GetActorLocation` (`self.Character`)) (`self.K2_GetActorLocation`))) 145.0))
        (`self.K2_AddActorWorldRotation` (`KismetMathLibrary.MakeRotator` 0.0 0.0 (`self.Find Rotate`)))
        (set `self.PreviousRotate` (`self.K2_GetActorRotation`))
        (set `self.PreviousLocation` (`self.K2_GetActorLocation`))
        (set `self.PreviousForwardVector` (`self.GetActorForwardVector`))
        (bind (_direction _yaw _location) (`Timeline|RotateCube` :!via `PlayFromStart`)
          (:`Update`
            (`self.K2_SetActorRotation` (`KismetMathLibrary.MakeRotator` 0.0 (+ (`KismetMathLibrary.Lerp` 0.0 90.0 _yaw) _previousrotate_pitch_2) _previousrotate_yaw))
            (`self.K2_SetActorLocation` (+ (`self.PreviousLocation`) (* (`self.PreviousForwardVector`) (.y _location)) (`KismetMathLibrary.MakeVector` 0.0 0.0 (.z _location)))))
          (:`Finished`
            (`self.K2_SetActorRotation` (`KismetMathLibrary.MakeRotator` 0.0 _previousrotate_pitch (`self.StartRotationYaw`)))
            (`GameplayStatics.PlaySound2D` "/Game/StealthShooter/Assets/Sound/A_BoxImpact.A_BoxImpact" 1.0 1.0 0.0 null null)
            (goto _label :!via `Reset`)))
        (else
          (goto _label :!via `Reset`))))))

(fn `CheckObstacle`
  (params (Rotate :type "Float (double-precision)"))
  (returns (Obstacle :type Boolean))
  (bind (_returnvalue_roll _returnvalue_pitch _returnvalue_yaw) (`KismetMathLibrary.BreakRotator` (`self.K2_GetActorRotation`)))
  (bind _returnvalue (+ Rotate _returnvalue_yaw))
  (bind _returnvalue_2 (+ (`self.K2_GetActorLocation`) (* (`KismetMathLibrary.GetForwardVector` (`KismetMathLibrary.MakeRotator` 0.0 0.0 _returnvalue)) -200.0)))
  ;[0 0 0] Проверка на препятствия
  (bind (_outhit _returnvalue_3) (`KismetSystemLibrary.BoxTraceSingle` :`Start` _returnvalue_2 :`End` _returnvalue_2 :`HalfSize` (95.0 95.0 80.0) :`Orientation` (`KismetMathLibrary.MakeRotator` _returnvalue_roll _returnvalue_pitch _returnvalue) :`TraceChannel` "TraceTypeQuery1" :`bIgnoreSelf` false))
  (return _returnvalue_3))

(fn `Find Rotate`
  (returns (Rotate :type "Float (single-precision)"))
  (bind (_returnvalue_roll _returnvalue_pitch _returnvalue_yaw) (`KismetMathLibrary.BreakRotator` (`KismetMathLibrary.FindRelativeLookAtRotation` (`self.GetTransform`) (`self.K2_GetActorLocation` (`self.Character`)))))
  ;[0 0 0] Поиск поворота куба по Z
  (return (select `int` (`KismetMathLibrary.Round` (`KismetMathLibrary.SelectFloat` (`KismetMathLibrary.MapRangeClamped` _returnvalue_yaw 0.0 180.0 3.0 5.0) (`KismetMathLibrary.MapRangeClamped` _returnvalue_yaw 0.0 -180.0 0.0 2.0) (> _returnvalue_yaw 0.0))) :`0` 0.0 :`1` -90.0 :`2` 180.0 :`3` 0.0 :`4` 90.0 :`5` 180.0 :!type "Float (single-precision)")))

(fn `UserConstructionScript`)