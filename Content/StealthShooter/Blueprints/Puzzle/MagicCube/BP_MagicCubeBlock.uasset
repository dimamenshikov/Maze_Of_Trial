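; BP_MagicCubeBlock is a magic cube puzzle block whose height follows the sum of numbers from nearby platforms.
; On BeginPlay, a line trace scaled and rotated with the block finds BP_MagicCubePlatform actors and binds to their number events.
; Each event adds to the running sum, which maps unclamped to a vertical offset from the start position.
; A next-tick delay loop moves the block there at constant speed, without Event Tick.
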(event `self.ReceiveBeginPlay`
  (bind _returnvalue (`self.K2_GetActorLocation`))
  (bind _returnvalue_2 (`self.K2_GetActorRotation`))
  (bind _returnvalue_3 (`self.GetActorScale3D`))
  ;[0 0 0] Привязка события к плитам, движение в зависимости от суммы чисел на плитах
  (set `self.StartLocation` (`self.K2_GetActorLocation`))
  (bind _outhits (`KismetSystemLibrary.LineTraceMulti` (+ (`KismetMathLibrary.GreaterGreater_VectorRotator` (* (`self.StartTrace`) _returnvalue_3) _returnvalue_2) _returnvalue) (+ _returnvalue (`KismetMathLibrary.GreaterGreater_VectorRotator` (* _returnvalue_3 (`self.EndTrace`)) _returnvalue_2)) "TraceTypeQuery1"))
  (for _array_element _outhits
    (bind _asbp_magic_cube_platform (cast `/Game/StealthShooter/Blueprints/Puzzle/MagicCube/BP_MagicCubePlatform` (`.HitActor` (`GameplayStatics.BreakHitResult` _array_element))))
    (add `/Game/StealthShooter/Blueprints/Puzzle/MagicCube/BP_MagicCubePlatform.OnNumberCube` _asbp_magic_cube_platform (delegate `SetSumm`))))

(event `SetSumm`
  (params (Index :type Integer))
  (bind (_returnvalue_x _returnvalue_y _returnvalue_z) (`KismetMathLibrary.BreakVector` (`self.K2_GetActorLocation`)))
  (bind (_startlocation_x _startlocation_y _startlocation_z) (`KismetMathLibrary.BreakVector` (`self.StartLocation`)))
  ;[0 0 0] Привязка события к плитам, движение в зависимости от суммы чисел на плитах
  (bind _output_get (set `self.Summ` (+ Index (`self.Summ`))))
  (bind _returnvalue (+ _startlocation_z (`KismetMathLibrary.MapRangeUnclamped` (`KismetMathLibrary.Conv_IntToDouble` _output_get) 0.0 15.0 0.0 -185.0)))
  (`self.K2_SetActorLocation` (`KismetMathLibrary.MakeVector` _returnvalue_x _returnvalue_y (`KismetMathLibrary.FInterpTo_Constant` _returnvalue_z _returnvalue (`GameplayStatics.GetWorldDeltaSeconds`) 30.0)) :!label _label)
  (if (not (== _returnvalue_z _returnvalue))
    (`KismetSystemLibrary.DelayUntilNextTick`)
    (goto _label)))

(fn `UserConstructionScript`)