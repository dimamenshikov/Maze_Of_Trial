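; Numbered cube for the Magic Cube puzzle that the player picks up and drops by interacting.
; A FlipFlop alternates between attaching it to the character, if nothing else is attached, and detaching it with physics enabled.
; Each successful toggle fires OnActive with the negated Number on pickup or the positive Number on drop.
; The construction script visualizes Number with small instanced meshes at 45-degree steps, alternating radii to form a square.
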(event `self.ReceiveBeginPlay`
  ;[0 0 0] Сохранение нужных ссылок в переменные
  (bind _asbp_character (cast `/Game/StealthShooter/Blueprints/Core/Character/BP_Character` (`GameplayStatics.GetPlayerPawn` 0)))
  (set `self.Character` _asbp_character)
  (set `self.StartLocation` (`self.K2_GetActorLocation`)))

(event `/Game/StealthShooter/Blueprints/Interface/BPI_Interaction.Interaction`
  (params (On :type Boolean))
  (bind _block (`self.Block`))
  (bind _character (`self.Character`))
  ;[0 0 0] Прикрепление или открепление куба к персонажу
  (`/Engine/EditorBlueprintResources/StandardMacros.FlipFlop`
    (:`A`
      (if (`KismetArrayLibrary.Array_IsEmpty` (`self.GetAttachedActors` _character true false))
        (`self.K2_AttachToActor` _character "None" "KeepRelative" "KeepWorld" "KeepWorld")
        (`self.K2_SetActorRelativeLocation` (90.0 0.0 20.0))
        (set `self.bActive` false)
        (`self.OnActive` false (* (`self.Number`) -1))))
    (:`B`
      (if (!= (`KismetArrayLibrary.Array_Find` (`self.GetAttachedActors` (`self.Character`) false false) self) -1)
        (`self.K2_DetachFromActor` "KeepWorld" "KeepWorld" "KeepWorld")
        (`PrimitiveComponent.SetCollisionEnabled` _block "PhysicsOnly")
        (`PrimitiveComponent.SetSimulatePhysics` _block true)
        (set `self.bActive` true)
        (`self.OnActive` true (`self.Number`))))))

(fn `UserConstructionScript`
  ;[0 0 0] Создание количества кубов в зависимости от номера
  (bind _returnvalue (`AddComponent|NODE_AddInstancedStaticMeshComponent-0`))
  (set `self.Cubes` _returnvalue)
  (for _index (range 2 (+ (`self.Number`) 1))
    (`InstancedStaticMeshComponent.AddInstance` (`self.Cubes`) (`KismetMathLibrary.MakeTransform` (`KismetMathLibrary.GreaterGreater_VectorRotator` (`KismetMathLibrary.MakeVector` (`KismetMathLibrary.SelectFloat` 42.0 59.22 (== (mod _index 2) 0))) (`KismetMathLibrary.MakeRotator` 0.0 0.0 (* _index 45.0))) (struct) (0.4 0.4 0.4)) false)))