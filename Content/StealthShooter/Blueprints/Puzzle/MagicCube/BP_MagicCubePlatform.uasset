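; BP_MagicCubePlatform is a magic cube puzzle platform that accepts a numbered cube and reports its number to listeners.
; Box overlaps track the cube, bind to its OnActive event and call UpDown, passing a negated number on exit.
; Placement snaps the cube to the box, and a timeline lowers the platform with gate audio, then disables the block's physics and collision.
; Removal reverses the timeline, with OnCube and a DoOnce gating state changes.
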(event `self.ReceiveBeginPlay`
  ;[0 0 0] Создание звука
  (bind _returnvalue (`GameplayStatics.CreateSound2D` "/Game/StealthShooter/Assets/Sound/A_Gate.A_Gate" 0.0 1.0 0.0 null false false))
  (bind _output_get (set `self.Sound` _returnvalue))
  (`KismetSystemLibrary.Delay` 1.0)
  (`AudioComponent.SetVolumeMultiplier` _output_get 1.0))

(event `UpDown`
  (params (Down :type Boolean) (Index :type Integer))
  (bind _sound (`self.Sound`))
  (bind (_returnvalue_location _returnvalue_rotation) (`KismetMathLibrary.BreakTransform` (`SceneComponent.K2_GetComponentToWorld` (`self.Box`))))
  (bind _block (`/Game/StealthShooter/Blueprints/Puzzle/MagicCube/BP_MagicCubeNumberCube.Block` (`self.NumberCube`)))
  ;[0 0 0] Прикрепление куба к платформе
  (if (`/Game/StealthShooter/Blueprints/Puzzle/MagicCube/BP_MagicCubeNumberCube.bActive` (`self.NumberCube`))
    (`|ExecutionSequence`
      (:`then_0`
        (goto _label_3 :!via `Reset`))
      (:`then_1`
        (if (not (`self.bOnCube`))
          (set `/Game/StealthShooter/Blueprints/Puzzle/MagicCube/BP_MagicCubeNumberCube.bActive` false (`self.NumberCube`))
          (`self.OnNumberCube` Index)
          (`PrimitiveComponent.SetPhysicsLinearVelocity` (`/Game/StealthShooter/Blueprints/Puzzle/MagicCube/BP_MagicCubeNumberCube.Block` (`self.NumberCube`)) (0.0 0.0 0.0) false "None")
          (`self.K2_SetActorLocationAndRotation` (`self.NumberCube`) _returnvalue_location _returnvalue_rotation false false)
          (set `self.bOnCube` true)
          (`AudioComponent.SetPaused` _sound false :!label _label)
          (`AudioComponent.Play` _sound 0.0)
          ;[0 0 0] Поднимание или опускание платформы
          (if Down
            (bind (_direction _locationz) (`Timeline|OffsetUpDown` :!label _label_2)
              (:`Update`
                (`SceneComponent.K2_SetRelativeLocation` (`self.Cube`) (`KismetMathLibrary.MakeVector` 0.0 0.0 _locationz) false false))
              (:`Finished`
                (`AudioComponent.SetPaused` (`self.Sound`) true)
                (if (`|EnumEquality` _direction "Forward")
                  (`PrimitiveComponent.SetSimulatePhysics` _block false)
                  (`PrimitiveComponent.SetCollisionEnabled` _block "NoCollision"))))
            (else
              (set `self.bOnCube` false)
              (goto _label_2 :!via `Reverse`))))))
    (elif (`self.bOnCube`)
      (`/Engine/EditorBlueprintResources/StandardMacros.DoOnce` false :!label _label_3
        (:`Completed`
          (set `self.bOnCube` false)
          (`self.OnNumberCube` Index)
          (goto _label))))))

(event `self.Box.OnComponentBeginOverlap`
  (params (OverlappedComponent :type "PrimitiveComponent Object Reference") (OtherActor :type "Actor Object Reference") (OtherComp :type "PrimitiveComponent Object Reference") (OtherBodyIndex :type Integer) (bFromSweep :type Boolean) (SweepResult :type "HitResult Structure (by ref)"))
  ;[0 0 0] Вызов опускания платформы
  (if (not (`self.bOnCube`))
    (bind _asbp_magic_cube_number_cube (cast `/Game/StealthShooter/Blueprints/Puzzle/MagicCube/BP_MagicCubeNumberCube` OtherActor))
    (bind _output_get (set `self.NumberCube` _asbp_magic_cube_number_cube))
    (`KismetSystemLibrary.DelayUntilNextTick`)
    (add `/Game/StealthShooter/Blueprints/Puzzle/MagicCube/BP_MagicCubeNumberCube.OnActive` _output_get (`|CreateDelegate` :!event `UpDown`))
    (if (`/Game/StealthShooter/Blueprints/Puzzle/MagicCube/BP_MagicCubeNumberCube.bActive` _output_get)
      (`self.UpDown` true (`/Game/StealthShooter/Blueprints/Puzzle/MagicCube/BP_MagicCubeNumberCube.Number` _output_get)))))

(event `self.Box.OnComponentEndOverlap`
  (params (OverlappedComponent :type "PrimitiveComponent Object Reference") (OtherActor :type "Actor Object Reference") (OtherComp :type "PrimitiveComponent Object Reference") (OtherBodyIndex :type Integer))
  ;[0 0 0] Вызов поднятия платформы
  (bind _asbp_magic_cube_number_cube (cast `/Game/StealthShooter/Blueprints/Puzzle/MagicCube/BP_MagicCubeNumberCube` OtherActor))
  (if (== _asbp_magic_cube_number_cube (`self.NumberCube`))
    (`KismetSystemLibrary.DelayUntilNextTick`)
    (remove `/Game/StealthShooter/Blueprints/Puzzle/MagicCube/BP_MagicCubeNumberCube.OnActive` _asbp_magic_cube_number_cube (`|CreateDelegate` :!event `UpDown`))
    (if (`/Game/StealthShooter/Blueprints/Puzzle/MagicCube/BP_MagicCubeNumberCube.bActive` _asbp_magic_cube_number_cube)
      (`self.UpDown` false (* (`/Game/StealthShooter/Blueprints/Puzzle/MagicCube/BP_MagicCubeNumberCube.Number` _asbp_magic_cube_number_cube) -1)))))

(fn `UserConstructionScript`)