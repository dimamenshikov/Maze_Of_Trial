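; Possessable pawn for the DodgeBomb puzzle that the player enters and leaves through an alternating Interaction event.
; Entering hides the roof and character, attaches the character to the UFO at an offset facing the pawn, and possesses the pawn with look input locked and control rotation taken from the camera's up vector.
; Exiting reverses this and restores character collision.
; While active, Tick smoothly rotates the pawn toward its velocity.
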(event `self.ReceiveBeginPlay`
  ;[0 0 0] Сохранение нужных ссылок в переменные
  (bind _asbp_player_controller_maze (cast `/Game/StealthShooter/Blueprints/Core/PlayerController/BP_PlayerControllerMaze` (`GameplayStatics.GetPlayerController` 0)))
  (set `self.PlayerControllerMaze` _asbp_player_controller_maze)
  (bind _asbp_character (cast `/Game/StealthShooter/Blueprints/Core/Character/BP_Character` (`GameplayStatics.GetPlayerPawn` 0)))
  (set `self.Character` _asbp_character))

(event `/Game/StealthShooter/Blueprints/Interface/BPI_Interaction.Interaction`
  (params (On :type Boolean))
  (bind _roof (`self.Roof`))
  (bind _playercontrollermaze (`self.PlayerControllerMaze`))
  (bind _playercontrollermaze_2 (`self.PlayerControllerMaze`))
  (bind _character (`self.Character`))
  (bind (_returnvalue_roll _returnvalue_pitch _returnvalue_yaw) (`KismetMathLibrary.BreakRotator` (`KismetMathLibrary.FindLookAtRotation` (`self.K2_GetActorLocation` (`self.Character`)) (`self.K2_GetActorLocation`))))
  (bind (_returnvalue_x _returnvalue_y) (`KismetMathLibrary.BreakVector` (- (`self.K2_GetActorLocation` (`self.Character`)) (`self.K2_GetActorLocation`))))
  (bind (_returnvalue_x_2 _returnvalue_y_2) (`KismetMathLibrary.BreakVector` (* (`KismetMathLibrary.Normal` (`KismetMathLibrary.MakeVector` _returnvalue_x _returnvalue_y)) 300.0)))
  ;[0 0 0] Привязка контроллера к актору
  (`/Engine/EditorBlueprintResources/StandardMacros.FlipFlop`
    (:`A`
      (`self.SetActorHiddenInGame` _roof true)
      (`self.SetActorHiddenInGame` (`self.Character`) true)
      (`self.K2_AttachToComponent` (`self.Character`) (`self.UFO`) "None" "KeepWorld" "KeepWorld" "KeepWorld" false)
      (`self.K2_SetActorRelativeLocation` (`self.Character`) (`KismetMathLibrary.MakeVector` _returnvalue_x_2 _returnvalue_y_2 90.0) false false)
      (`self.K2_SetActorRotation` (`self.Character`) (`KismetMathLibrary.MakeRotator` 0.0 0.0 _returnvalue_yaw) false)
      (`Controller.Possess` _playercontrollermaze_2 self)
      (`Controller.SetIgnoreLookInput` _playercontrollermaze_2 true)
      (`Controller.SetControlRotation` _playercontrollermaze_2 (`KismetMathLibrary.MakeRotFromX` (`SceneComponent.GetUpVector` (`self.Camera`))))
      (set `/Game/StealthShooter/Blueprints/Core/Character/BP_Character.bPawn` true (`self.Character`)))
    (:`B`
      (`self.SetActorHiddenInGame` _roof false)
      (`self.SetActorHiddenInGame` (`self.Character`) false)
      (`self.K2_DetachFromActor` _character "KeepWorld" "KeepWorld" "KeepWorld")
      (`PrimitiveComponent.SetCollisionEnabled` (`Character.CapsuleComponent` _character) "QueryAndPhysics")
      (`Controller.Possess` _playercontrollermaze (`self.Character`))
      (`Controller.SetIgnoreLookInput` _playercontrollermaze false)
      (set `/Game/StealthShooter/Blueprints/Core/Character/BP_Character.bPawn` false (`self.Character`)))))

(event `self.ReceiveTick`
  (params (DeltaSeconds :type "Float (single-precision)"))
  (bind _returnvalue (`self.GetVelocity`))
  ;[0 0 0] Поворот актора по направлению движения
  (if (and (`/Game/StealthShooter/Blueprints/Core/Character/BP_Character.bPawn` (`self.Character`)) (!= _returnvalue (0.0 0.0 0.0) :`ErrorTolerance` 0.01))
    (`self.K2_SetActorRotation` (`KismetMathLibrary.RInterpTo` (`self.K2_GetActorRotation`) (`KismetMathLibrary.Conv_VectorToRotator` _returnvalue) (`GameplayStatics.GetWorldDeltaSeconds`) 8.0))))

(fn `UserConstructionScript`)