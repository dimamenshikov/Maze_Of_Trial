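; BP_Teleport is a moving portal that teleports the player character or Pawn-tagged actors to TeleportLocation on overlap and plays a portal sound.
; While active, a timeline loops it through its points, yawing it toward the player.
; BeginPlay converts local points to world space, appends the start location and sets segment speed from Time.
; LoadGame activates it; Activate also toggles an "Active" tag.
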(event `/Game/StealthShooter/Blueprints/Interface/BPI_SaveGame.LoadGame`
  ;[0 0 0] Активирование при загрузки уровня
  (`/Game/StealthShooter/Blueprints/Interface/BPI_Interaction.Activate` true))

(event `/Game/StealthShooter/Blueprints/Interface/BPI_Interaction.Activate`
  (params (Activate :type Boolean))
  (bind _tags (`self.Tags`))
  (bind _returnvalue (+ (`self.Index`) 1))
  (bind (_returnvalue_roll _returnvalue_pitch _returnvalue_yaw) (`KismetMathLibrary.BreakRotator` (`KismetMathLibrary.FindLookAtRotation` (`self.K2_GetActorLocation`) (`self.K2_GetActorLocation` (`GameplayStatics.GetPlayerPawn` 0)))))
  ;[0 0 0] Движение телепорта по точкам
  (if Activate
    (`KismetArrayLibrary.Array_Add` _tags "Active")
    (else
      (`KismetArrayLibrary.Array_RemoveItem` _tags "Active")))
  (if Activate :!label _label
    (set `self.StartLocation` (`|GetArrayItem` (`self.Points`) (`self.Index`)))
    (bind _output_get (set `self.Index` (`KismetMathLibrary.SelectInt` _returnvalue 0 (< _returnvalue (`KismetArrayLibrary.Array_Length` (`self.Points`))))))
    (set `self.EndPoint` (`|GetArrayItem` (`self.Points`) _output_get))
    (bind (_direction _alpha) (`Timeline|Move` :!via `PlayFromStart`)
      (:`Update`
        (`self.K2_SetActorLocation` (`KismetMathLibrary.VLerp` (`self.StartLocation`) (`self.EndPoint`) _alpha))
        (`self.K2_SetActorRotation` (`KismetMathLibrary.MakeRotator` 0.0 0.0 (- _returnvalue_yaw 90.0))))
      (:`Finished`
        (`KismetSystemLibrary.DelayUntilNextTick`)
        (goto _label)))))

(event `self.ReceiveBeginPlay`
  ;[0 0 0] Перевод локальных координат точек в мировые
  (`TimelineComponent.SetPlayRate` (`self.Move`) (/ 1.0 (`self.Time`)))
  (for (_array_element _array_index) (`self.Points`)
    (`KismetArrayLibrary.Array_Set` (`self.Points`) _array_index (+ (`KismetMathLibrary.GreaterGreater_VectorRotator` (* _array_element (`self.GetActorScale3D`)) (`self.K2_GetActorRotation`)) (`self.K2_GetActorLocation`))))
  (`KismetArrayLibrary.Array_Add` (`self.Points`) (`self.K2_GetActorLocation`)))

(event `self.Box.OnComponentBeginOverlap`
  (params (OverlappedComponent :type "PrimitiveComponent Object Reference") (OtherActor :type "Actor Object Reference") (OtherComp :type "PrimitiveComponent Object Reference") (OtherBodyIndex :type Integer) (bFromSweep :type Boolean) (SweepResult :type "HitResult Structure (by ref)"))
  (bind _returnvalue (`self.ActorHasTag` OtherActor "Pawn"))
  ;[0 0 0] Телепортация персонажа и проигрывание звука
  (bind _asbp_character (cast `/Game/StealthShooter/Blueprints/Core/Character/BP_Character` OtherActor)
    (:`then`
      (if (not (`/Game/StealthShooter/Blueprints/Core/Character/BP_Character.bPawn` _asbp_character))
        (`self.K2_SetActorLocation` OtherActor (+ (`self.TeleportLocation`) (`KismetMathLibrary.SelectVector` (0.0 0.0 0.0) (0.0 0.0 100.0) _returnvalue)) false true :!label _label_2)
        (`GameplayStatics.PlaySound2D` "/Game/StealthShooter/Assets/Sound/A_Portal.A_Portal" 1.0 1.0 0.0 null null)))
    (:`CastFailed`
      (if _returnvalue
        (goto _label_2)))))

(fn `UserConstructionScript`)