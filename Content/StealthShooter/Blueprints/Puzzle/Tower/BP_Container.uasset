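; BP_Container is a tower-puzzle container that punishes the player for stacking it on a smaller one.
; CheckLocation box-traces for another container and compares X scales; if that one is smaller, both play Destroy and the player takes delayed damage.
; A shared timeline animates the smaller container's scale and the larger one's height, then spawns explosions at the player and hides both.
; The GameMode's player rebirth event restores visibility and starting transforms.
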(event `self.ReceiveBeginPlay`
  (bind _sm_cornerframe (`self.SM_CornerFrame`))
  ;[0 0 0] Сохранение начальной трансформации, масштаба, привязка к событию возрождения персонажа
  (set `self.StartTransform` (`self.GetTransform`))
  (set `self.Scale` (`SceneComponent.RelativeScale3D` _sm_cornerframe))
  (set `self.StartRelativeTransform` (`SceneComponent.GetRelativeTransform` _sm_cornerframe))
  (bind _asbp_game_mode_maze (cast `/Game/StealthShooter/Blueprints/Core/GameModes/BP_GameModeMaze` (`GameplayStatics.GetGameMode`)))
  (add `/Game/StealthShooter/Blueprints/Core/GameModes/BP_GameModeMaze.OnRebirthPlayer` _asbp_game_mode_maze (delegate `Restart`)))

(event `Restart`
  ;[0 0 0] Сохранение начальной трансформации, масштаба, привязка к событию возрождения персонажа
  (`self.SetActorHiddenInGame` false)
  (`self.K2_SetActorTransform` (`self.StartTransform`) false true)
  (`SceneComponent.K2_SetRelativeTransform` (`self.SM_CornerFrame`) (`self.StartRelativeTransform`) false false))

(event `CheckLocation`
  (bind _returnvalue_x (`KismetMathLibrary.BreakVector` (`self.GetActorScale3D`)))
  (bind _returnvalue (`self.K2_GetActorLocation`))
  (bind _scale_x (`KismetMathLibrary.BreakVector` (`self.Scale`)))
  (bind _returnvalue_2 (* _scale_x 10.0))
  ;[0 0 0] Проверка контейнера внизу, если снизу меньше, то вызов уничтожения обоих контейнеров и персонажа
  (`GameplayStatics.PlaySound2D` "/Game/StealthShooter/Assets/Sound/A_BoxImpact.A_BoxImpact" 1.0 1.0 0.0 null null)
  (bind _outhit (`KismetSystemLibrary.BoxTraceSingle` _returnvalue _returnvalue (`KismetMathLibrary.MakeVector` _returnvalue_2 _returnvalue_2 25.0) (`self.K2_GetActorRotation`) "TraceTypeQuery1"))
  (bind _asbp_container (cast `/Game/StealthShooter/Blueprints/Puzzle/Tower/BP_Container` (`.HitActor` (`GameplayStatics.BreakHitResult` _outhit))))
  (bind _returnvalue_x_2 (`KismetMathLibrary.BreakVector` (`self.GetActorScale3D` _asbp_container)))
  (if (< _returnvalue_x_2 _returnvalue_x)
    (`self.Destroy` _asbp_container true)
    (`self.Destroy` false)
    (`KismetSystemLibrary.Delay` 2.1)
    (`GameplayStatics.ApplyDamage` (`GameplayStatics.GetPlayerPawn` 0) 100.0)
    (`GameplayStatics.PlaySound2D` "/Game/StealthShooter/Assets/Sound/A_Explosion.A_Explosion" 1.0 1.0 0.0 null null)))

(event `Destroy`
  (params (Less :type Boolean))
  (bind _scale (`self.Scale`))
  (bind _sm_cornerframe (`self.SM_CornerFrame`))
  (bind (_currentlocation_x _currentlocation_y _currentlocation_z) (`KismetMathLibrary.BreakVector` (`self.CurrentLocation`)))
  (bind _relativescale3d_x (`KismetMathLibrary.BreakVector` (`SceneComponent.RelativeScale3D` (`self.SM_CornerFrame`))))
  ;[0 0 0] Уничтожение персонажа и сокрытие контейнеров
  (set `self.CurrentLocation` (`SceneComponent.K2_GetComponentLocation` (`self.SM_CornerFrame`)))
  (bind (_direction _scale_2 _locationz) (`Timeline|OffsetTransform` :!via `PlayFromStart`)
    (:`Update`
      (`SceneComponent.SetRelativeScale3D` _sm_cornerframe (`KismetMathLibrary.SelectVector` (* _scale _scale_2) _scale Less))
      (`SceneComponent.K2_SetWorldLocation` _sm_cornerframe (`KismetMathLibrary.MakeVector` _currentlocation_x _currentlocation_y (`KismetMathLibrary.SelectFloat` _currentlocation_z (+ _currentlocation_z _locationz) Less)) false false))
    (:`Finished`
      (`GameplayStatics.SpawnEmitterAtLocation` "/Game/StealthShooter/Assets/Effects/Explosion/PS_Explosion.PS_Explosion" (`self.K2_GetActorLocation` (`GameplayStatics.GetPlayerPawn` 0)) (struct) (`KismetMathLibrary.MakeVector` _relativescale3d_x _relativescale3d_x _relativescale3d_x))
      (`self.SetActorHiddenInGame` true))))

(fn `UserConstructionScript`)