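; Puzzle crane that carries a BP_Container from one queued point to another, with lamp events and looping motion steps.
; Once two locations are queued, it slides the Kernel along Y, then stretches its Z scale to a downward trace's distance to lower and raise.
; Box overlap attaches the container at the first stop; the second detaches it and calls CheckLocation.
; Next-tick delay loops drive motion; player rebirth restores the Kernel transform.
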(event `self.ReceiveBeginPlay`
  ;[0 0 0] Сохранение начальной трансформации, привязка события на возрождение персонажа, создание звука
  (set `self.StartRelativeTransform` (`SceneComponent.GetRelativeTransform` (`self.Kernel`)))
  (bind _asbp_game_mode_maze (cast `/Game/StealthShooter/Blueprints/Core/GameModes/BP_GameModeMaze` (`GameplayStatics.GetGameMode`)))
  (add `/Game/StealthShooter/Blueprints/Core/GameModes/BP_GameModeMaze.OnRebirthPlayer` _asbp_game_mode_maze (delegate `Restart`))
  (bind _returnvalue (`GameplayStatics.CreateSound2D` "/Game/StealthShooter/Assets/Sound/A_Crane.A_Crane" 1.0 1.0 0.0 null false false))
  (set `self.SoundCrane` _returnvalue))

(event `Restart`
  ;[0 0 0] Сохранение начальной трансформации, привязка события на возрождение персонажа, создание звука
  (`SceneComponent.K2_SetRelativeTransform` (`self.Kernel`) (`self.StartRelativeTransform`) false true))

(event `Down`
  (bind _scene (`self.Scene`))
  (bind _returnvalue (`SceneComponent.K2_GetComponentLocation` _scene))
  (bind (_relativescale3d_x _relativescale3d_y _relativescale3d_z) (`KismetMathLibrary.BreakVector` (`SceneComponent.RelativeScale3D` (`self.Kernel`))))
  ;[0 0 0] Опускание, поднимание крана, открепление контейнера
  (bind _outhit (`KismetSystemLibrary.LineTraceSingle` _returnvalue (+ _returnvalue (* (`SceneComponent.GetUpVector` _scene) -3000.0)) "TraceTypeQuery1" false (`|MakeArray` (`self.Container`) :!type "Actor Object Reference")))
  (cast `/Game/StealthShooter/Blueprints/Puzzle/Tower/BP_Container` (`.HitActor` (`GameplayStatics.BreakHitResult` _outhit))
    (:`then`
      (bind _returnvalue_2 (+ (/ (`.Distance` (`GameplayStatics.BreakHitResult` _outhit)) 100.0) 1.0))
      (bind _output_get (set `self.End` (+ _returnvalue_2 (`KismetMathLibrary.SelectFloat` 1.0 0.0 (== (`self.Index`) 0))))))
    (:`CastFailed`
      (set `self.End` _returnvalue_2)))
  (`SceneComponent.SetRelativeScale3D` (`self.Kernel`) (`KismetMathLibrary.MakeVector` 0.1 0.1 (`KismetMathLibrary.FInterpTo_Constant` _relativescale3d_z _output_get (`GameplayStatics.GetWorldDeltaSeconds`) 15.0)) :!label _label)
  (if (== _relativescale3d_z _output_get)
    (`/Engine/EditorBlueprintResources/StandardMacros.FlipFlop`
      (:`A`
        (if (and (`KismetSystemLibrary.IsValid` (`self.Container`)) (== (`self.Index`) 1))
          (bind _container (`self.Container`)
            (:`then`
              (`self.K2_DetachFromActor` _container "KeepWorld" "KeepWorld" "KeepWorld")
              (`/Game/StealthShooter/Blueprints/Puzzle/Tower/BP_Container.CheckLocation` _container))
            (:`else`)))
        (set `self.End` 1.0)
        (goto _label))
      (:`B`
        (bind _result (`/Engine/EditorBlueprintResources/StandardMacros.IncrementInt` (`self.Index`))
          (:`  `
            (if (< _result 2)
              (`self.Movement` (`|GetArrayItem` (`self.EndTrace`) (`|GetArrayItem` (`self.Location`) (`self.Index`))))
              (else
                (`KismetArrayLibrary.Array_Clear` (`self.Location`))
                (set `self.Index` 0)
                (set `self.Container` null)
                (`self.OnLampOnOff` false)
                (`AudioComponent.SetPaused` (`self.SoundCrane`) true)))))))
    (else
      (`KismetSystemLibrary.DelayUntilNextTick`)
      (goto _label))))

(event `Move`
  (params (Location :type Integer))
  (bind _soundcrane (`self.SoundCrane`))
  ;[0 0 0] Вызов передвижения, загорание ламп, воспроизведение звука
  (bind _returnvalue (`KismetArrayLibrary.Array_Add` (`self.Location`) Location))
  (if (== _returnvalue 1)
    (`self.OnLampOnOff` true)
    (`AudioComponent.SetPaused` _soundcrane false)
    (`AudioComponent.Play` _soundcrane 4.1)
    (`self.Movement` (`|GetArrayItem` (`self.EndTrace`) (`|GetArrayItem` (`self.Location`) (`self.Index`))))))

(event `Movement`
  (params (Point :type "Vector Structure"))
  (bind (_relativelocation_x _relativelocation_y) (`KismetMathLibrary.BreakVector` (`SceneComponent.RelativeLocation` (`self.Kernel`))))
  ;[0 0 0] Передвижение крана, вызов опускания
  (`SceneComponent.K2_SetRelativeLocation` (`self.Kernel`) (`KismetMathLibrary.MakeVector` -5.0 (`KismetMathLibrary.FInterpTo_Constant` _relativelocation_y Point_Y (`GameplayStatics.GetWorldDeltaSeconds`) 1500.0) 100.0) false false :!label _label_2)
  (if (== _relativelocation_y Point_Y)
    (`self.Down`)
    (else
      (`KismetSystemLibrary.DelayUntilNextTick`)
      (goto _label_2))))

(event `self.Box.OnComponentBeginOverlap`
  (params (OverlappedComponent :type "PrimitiveComponent Object Reference") (OtherActor :type "Actor Object Reference") (OtherComp :type "PrimitiveComponent Object Reference") (OtherBodyIndex :type Integer) (bFromSweep :type Boolean) (SweepResult :type "HitResult Structure (by ref)"))
  (bind (_asbp_container _bsuccess) (cast `/Game/StealthShooter/Blueprints/Puzzle/Tower/BP_Container` OtherActor :!pure true))
  ;[0 0 0] Прикрепление контейнера к крану
  (if (and _bsuccess (== (`self.Index`) 0))
    (bind _output_get (set `self.Container` _asbp_container))
    (set `self.bOverlap` true)
    (`self.K2_AttachToComponent` _output_get (`self.Box`) "None" "KeepWorld" "KeepWorld" "KeepWorld" true)))

(fn `UserConstructionScript`)