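; BP_Plate is a plate in the TagGame sliding-tile puzzle, with an optional empty plate hidden in game.
; Construction creates a dynamic material, and BeginPlay stores the start location plus that of an optional copy plate, BCopy.
; Blick line-traces along a rotation-relative offset to hand the highlight color to a neighboring plate and returns the selected one.
; CheckLocation sets OnPlace when the plate sits at either stored location within tolerance.
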(event `self.ReceiveBeginPlay`
  ;[0 0 0] Сохранение начальной локации и локации плиты копии, если она есть
  (set `self.Start` (`self.K2_GetActorLocation`))
  (bind _bcopy (`self.bCopy`)
    (:`then`
      (set `self.StartCopy` (`self.K2_GetActorLocation` _bcopy)))
    (:`else`)))

(fn `Blick`
  (params (Offset :type "Vector2D Structure"))
  (returns (PlateActive :type "Self Object Reference"))
  (bind (_x _y) (`KismetMathLibrary.BreakVector2D` Offset))
  (bind _returnvalue (`KismetMathLibrary.GreaterGreater_VectorRotator` (`KismetMathLibrary.MakeVector` 0.0 (* _y 15.0) (* 15.0 _x)) (`KismetMathLibrary.ComposeRotators` (`self.K2_GetActorRotation`) (struct :`Yaw` -90.0))))
  (bind _returnvalue_2 (+ _returnvalue (`self.K2_GetActorLocation`)))
  ;[0 0 0] Передача подсветки выбранной плиты соседней плите
  (bind _outhit (`KismetSystemLibrary.LineTraceSingle` _returnvalue_2 (+ _returnvalue _returnvalue_2) "TraceTypeQuery1"))
  (bind _asbp_plate (cast `/Game/StealthShooter/Blueprints/Puzzle/TagGame/BP_Plate` (`.HitActor` (`GameplayStatics.BreakHitResult` _outhit)))
    (:`then`
      (`MaterialInstanceDynamic.SetVectorParameterValue` (`self.Material`) "Color" (struct :`R` 0.2 :`G` 0.2 :`B` 0.2 :`A` 1.0))
      (`MaterialInstanceDynamic.SetVectorParameterValue` (`/Game/StealthShooter/Blueprints/Puzzle/TagGame/BP_Plate.Material` _asbp_plate) "Color" (struct :`R` 0.5 :`G` 0.5 :`B` 0.5 :`A` 1.0))
      (return _asbp_plate))
    (:`CastFailed`
      (return self))))

(fn `CheckLocation`
  (bind _returnvalue (`self.K2_GetActorLocation`))
  (bind _returnvalue_2 (== (`self.Start`) _returnvalue :`ErrorTolerance` 0.1))
  ;[0 0 0] Проверка правильности позиции плиты
  (`self.bCopy`
    (:`then`
      (set `self.bOnPlace` (or _returnvalue_2 (== _returnvalue (`self.StartCopy`) :`ErrorTolerance` 0.1))))
    (:`else`
      (set `self.bOnPlace` _returnvalue_2))))

(fn `UserConstructionScript`
  ;[0 0 0] Создание динамического материала плиты и сокрытие пустой плиты
  (bind _returnvalue (`PrimitiveComponent.CreateDynamicMaterialInstance` (`self.Cube`) 0 null "None"))
  (set `self.Material` _returnvalue)
  (`SceneComponent.SetHiddenInGame` (`self.Cube`) (`self.bEmpty`) false))