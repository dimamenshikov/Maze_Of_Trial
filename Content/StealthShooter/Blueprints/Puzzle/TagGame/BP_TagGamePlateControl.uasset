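; Controller for a fifteen-style sliding plate puzzle that activates linked actors when solved.
; On BeginPlay it gathers all BP_Plate actors, randomly swaps eligible ones and records the empty slot.
; Interaction toggles puzzle mode, swapping Enhanced Input contexts, hiding the character and moving its camera.
; Player controller events drive plate highlighting and adjacent swaps with the empty slot; once every plate is in place, it unbinds them and messages the actors.
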(event `self.ReceiveBeginPlay`
  (bind _output (`|GetArrayItem` (`self.Plates`) (`self.Count`)))
  ;[0 0 0] Сохранение нужных ссылок в переменные сборка всех плит, перемешивание всех плит
  (`|ExecutionSequence`
    (:`then_0`
      (`KismetSystemLibrary.Delay` 0.2)
      (bind _asbp_character (cast `/Game/StealthShooter/Blueprints/Core/Character/BP_Character` (`GameplayStatics.GetPlayerPawn` 0)))
      (set `self.Character` _asbp_character))
    (:`then_1`
      (bind _asbp_player_controller_maze (cast `/Game/StealthShooter/Blueprints/Core/PlayerController/BP_PlayerControllerMaze` (`GameplayStatics.GetPlayerController` 0)))
      (bind _output_get (set `self.PlayerControllerMaze` _asbp_player_controller_maze))
      (add `/Game/StealthShooter/Blueprints/Core/PlayerController/BP_PlayerControllerMaze.OnOffsetPlate` _output_get (`|CreateDelegate` :!event `Offset`)))
    (:`then_2`
      (`KismetSystemLibrary.Delay` 1.0)
      (add `/Game/StealthShooter/Blueprints/Core/PlayerController/BP_PlayerControllerMaze.OnBlick` (`self.PlayerControllerMaze`) (`|CreateDelegate` :!event `Blick`))
      (bind _outactors (`GameplayStatics.GetAllActorsOfClass` "/Game/StealthShooter/Blueprints/Puzzle/TagGame/BP_Plate.BP_Plate_C"))
      (bind _output_get_2 (set `self.Plates` _outactors))
      (for _array_element _output_get_2
        (bind _output_get_3 (set `self.Count` (`KismetMathLibrary.RandomIntegerInRange` 0 16)))
        (if (and (`/Game/StealthShooter/Blueprints/Puzzle/TagGame/BP_Plate.bStartRandom` (`|GetArrayItem` (`self.Plates`) _output_get_3)) (`/Game/StealthShooter/Blueprints/Puzzle/TagGame/BP_Plate.bStartRandom` _array_element))
          (set `self.RandomChange` (`self.K2_GetActorLocation` _output))
          (`self.K2_SetActorLocation` _output (`self.K2_GetActorLocation` _array_element) false false)
          (`self.K2_SetActorLocation` _array_element (`self.RandomChange`) false false)))
      (set `self.Count` 0)
      (for (_array_element_2 _array_index) (`self.Plates`)
        (if (`/Game/StealthShooter/Blueprints/Puzzle/TagGame/BP_Plate.bEmpty` _array_element_2)
          (set `self.IndexEmpty` _array_index))
        (`/Game/StealthShooter/Blueprints/Puzzle/TagGame/BP_Plate.CheckLocation` _array_element_2)))))

(event `/Game/StealthShooter/Blueprints/Interface/BPI_Interaction.Interaction`
  (params (On :type Boolean))
  (bind _bplayernear (`self.bPlayerNear`))
  (bind _bplayernear_2 (`self.bPlayerNear`))
  (bind _returnvalue (not _bplayernear_2))
  (bind (_returnvalue_location _returnvalue_rotation) (`KismetMathLibrary.BreakTransform` (`SceneComponent.K2_GetComponentToWorld` (`self.Scene`))))
  (bind _returnvalue_2 (pcsubsystem `EnhancedInputLocalPlayerSubsystem` (`self.PlayerControllerMaze`)))
  (bind _returnvalue_3 (select `bool` _bplayernear_2 :`false` "/Game/StealthShooter/Blueprints/Input/IMC_Maze.IMC_Maze" :`true` "/Game/StealthShooter/Blueprints/Input/IMC_TagGame.IMC_TagGame" :!type "InputMappingContext Object Reference"))
  (bind _followcamera (`/Game/StealthShooter/Blueprints/Core/Character/BP_Character.FollowCamera` (`self.Character`)))
  ;[0 0 0] Активация управления пятнашками, перезапись системы управления у контроллера
  (`self.SetActorHiddenInGame` (`self.Character`) _returnvalue)
  (`EnhancedInputSubsystemInterface.RemoveMappingContext` _returnvalue_2 _returnvalue_3 (struct))
  (set `self.bPlayerNear` _returnvalue)
  (`EnhancedInputSubsystemInterface.AddMappingContext` _returnvalue_2 _returnvalue_3 0 (struct))
  (`Controller.SetIgnoreLookInput` (`self.PlayerControllerMaze`) _bplayernear)
  (if _bplayernear
    (`SceneComponent.K2_SetWorldLocationAndRotation` _followcamera _returnvalue_location _returnvalue_rotation false false)
    (else
      (`SceneComponent.K2_SetRelativeLocationAndRotation` :`self` _followcamera)
      (`MaterialInstanceDynamic.SetVectorParameterValue` (`/Game/StealthShooter/Blueprints/Puzzle/TagGame/BP_Plate.Material` (`|GetArrayItem` (`self.Plates`) (`self.Index`))) "Color" (struct :`R` 0.2 :`G` 0.2 :`B` 0.2 :`A` 1.0))))
  (set `/Game/StealthShooter/Blueprints/Core/PlayerController/BP_PlayerControllerMaze.MappingInput` (select `bool` _bplayernear :`false` "NewEnumerator0" :`true` "NewEnumerator1" :!type "/Game/StealthShooter/Blueprints/Enums/E_MappingInput Enum") (`self.PlayerControllerMaze`)))

(event `Blick`
  (params (X :type "Vector2D Structure"))
  (bind (_x _y) (`KismetMathLibrary.BreakVector2D` X))
  ;[0 0 0] Вызов подсветки у выбранной плиты
  (if (`self.bPlayerNear`)
    (bind _plateactive (`/Game/StealthShooter/Blueprints/Puzzle/TagGame/BP_Plate.Blick` (`|GetArrayItem` (`self.Plates`) (`self.Index`)) (`KismetMathLibrary.MakeVector2D` _x (`KismetMathLibrary.SelectFloat` _y 0.0 (== _x 0.0)))))
    (set `self.Index` (`KismetArrayLibrary.Array_Find` (`self.Plates`) _plateactive))))

(event `Offset`
  (bind _playercontrollermaze (`self.PlayerControllerMaze`))
  (bind _plates (`self.Plates`))
  (bind _output (`|GetArrayItem` (`self.Plates`) (`self.Index`)))
  (bind _output_2 (`|GetArrayItem` (`self.Plates`) (`self.IndexEmpty`)))
  (bind _returnvalue (`self.K2_GetActorLocation` (`|GetArrayItem` _plates (`self.IndexEmpty`))))
  (bind _returnvalue_2 (`self.K2_GetActorLocation` (`|GetArrayItem` _plates (`self.Index`))))
  (bind _material (`/Game/StealthShooter/Blueprints/Puzzle/TagGame/BP_Plate.Material` _output))
  ;[0 0 0] Перемещение плиты, проверка всех плит на правильность позиции, активация всех акторов
  (if (and (< (`KismetMathLibrary.VSize` (- _returnvalue_2 _returnvalue)) 55.0) (!= _returnvalue_2 _returnvalue :`ErrorTolerance` 0.1))
    (set `self.Empty` _returnvalue_2)
    (`self.K2_SetActorLocation` _output _returnvalue false true)
    (`self.K2_SetActorLocation` (`|GetArrayItem` (`self.Plates`) (`self.IndexEmpty`)) (`self.Empty`) false false)
    (`MaterialInstanceDynamic.SetVectorParameterValue` _material "Color" (struct :`R` 0.2 :`G` 0.2 :`B` 0.2 :`A` 1.0))
    (`MaterialInstanceDynamic.SetVectorParameterValue` _material "Color" (struct :`R` 0.5 :`G` 0.5 :`B` 0.5 :`A` 1.0))
    (`/Game/StealthShooter/Blueprints/Puzzle/TagGame/BP_Plate.CheckLocation` _output_2)
    (`GameplayStatics.PlaySound2D` "/Game/StealthShooter/Assets/Sound/A_PlateOffset.A_PlateOffset" 1.0 1.0 0.0 null null)
    (if (`/Game/StealthShooter/Blueprints/Puzzle/TagGame/BP_Plate.bOnPlace` _output_2)
      (set `self.bAllOnPlace` true)
      (for _array_element (`self.Plates`)
        (`/Game/StealthShooter/Blueprints/Puzzle/TagGame/BP_Plate.CheckLocation` _array_element)
        (if (not (`/Game/StealthShooter/Blueprints/Puzzle/TagGame/BP_Plate.bOnPlace` _array_element))
          (set `self.bAllOnPlace` false)
          (break)))
      (if (`self.bAllOnPlace`)
        (remove `/Game/StealthShooter/Blueprints/Core/PlayerController/BP_PlayerControllerMaze.OnBlick` _playercontrollermaze (`|CreateDelegate` :!event `Blick`))
        (remove `/Game/StealthShooter/Blueprints/Core/PlayerController/BP_PlayerControllerMaze.OnOffsetPlate` _playercontrollermaze (`|CreateDelegate` :!event `Offset`))
        (for _array_element_2 (`self.Actors`)
          (message `/Game/StealthShooter/Blueprints/Interface/BPI_Interaction.Activate` _array_element_2 true))))))

(fn `UserConstructionScript`)