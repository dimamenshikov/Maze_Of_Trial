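; Math helper function library that solves quadratic, cubic and quartic equations for real roots, with small time-formatting, sign and array utilities.
; The cubic solver branches on the discriminant sign into trigonometric or hyperbolic-style forms, using Math Expression nodes for the formulas.
; The quartic solver reduces to depressed form, takes a resolvent root from the cubic solver, then solves two quadratics, Ferrari-style.
; Array helpers remove duplicate roots and find a sign-filtered minimum or maximum.
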(fn TimeText
  (params (Time :type Float%20%28double-precision%29))
  ;[0 0 0] Отображение числа в формате времени
  (bind _output_get (LocalVariables|SetSeconds (Math|Float|%(Float) Time 6e+01)))
  (bind _output_get_2 (LocalVariables|SetMinutes (/ (Math|Float|%(Float) Time 3.6e+03) 60)))
  (return (Utilities|Text|FormatText "{Hours}:{Minutes}:{Seconds}" (/ Time 3.6e+03) (Utilities|String|SelectText (Utilities|Text|FormatText "0{Minutes}" _output_get_2) (Utilities|Text|ToText(Integer) _output_get_2) (< (LocalVariables|GetMinutes) 10)) (Utilities|String|SelectText (Utilities|Text|ToText(Float) _output_get "HalfToEven") (Utilities|Text|FormatText "0{Seconds}" (LocalVariables|GetSeconds)) (>= (LocalVariables|GetSeconds) 1e+01)))))

(fn SearchElementbyParamaters
  (params (Array :type Array%20of%20Floats%20%28double-precision%29) (Parameter :type E_SearchParameters%20Enum :default "NewEnumerator0") (Max :type Boolean))
  ;[0 0 0] Поиск минимального или максимального элемента в массиве среди элементов удовлетворяющих параметру
  (for _array_element Array
    (LocalVariables|SetArrayElement _array_element)
    (if (LocalVariables|GetFirstElement)
      (if (and (or (== (>= (LocalVariables|GetArrayElement) 0.0) (Utilities|Select :Index Parameter :NewEnumerator0 false :NewEnumerator1 false :NewEnumerator2 true)) (== 0 Parameter)) (== (<= (LocalVariables|GetElement) (LocalVariables|GetArrayElement)) Max))
        (LocalVariables|SetElement (LocalVariables|GetArrayElement) :!label _label))
      (else
        (LocalVariables|SetFirstElement (or (== (>= (LocalVariables|GetArrayElement) 0.0) (Utilities|Select :Index Parameter :NewEnumerator0 false :NewEnumerator1 false :NewEnumerator2 true)) (== 0 Parameter)))
        (goto _label))))
  (return (LocalVariables|GetFirstElement) (LocalVariables|GetElement)))

(fn DeleteDublicateRoots
  (params (Array :type Array%20of%20Floats%20%28double-precision%29))
  ;[0 0 0] Удаление одинаковых элементов в массиве
  (bind _output_get (LocalVariables|SetArrayLocal Array))
  (for (_array_element _array_index) _output_get
    (LocalVariables|SetElement _array_element)
    (LocalVariables|SetIndex (+ _array_index 1))
    (while (>= (Utilities|Array|LastIndex _output_get) (LocalVariables|GetIndex))
      (if (== (Utilities|Array|Get(acopy) (LocalVariables|GetArrayLocal) (LocalVariables|GetIndex)) (LocalVariables|GetElement))
        (Utilities|Array|RemoveIndex (LocalVariables|GetArrayLocal) (LocalVariables|GetIndex))
        (else
          (Math|Integer|IncrementInt (LocalVariables|GetIndex))))))
  (return (LocalVariables|GetArrayLocal)))

(fn SGN
  (params (Value :type Float%20%28double-precision%29))
  (return (Math|Float|Truncate (/ Value (Math|Float|Absolute(Float) Value)))))

(fn EducationSecondDegree
  (params (A :type Float%20%28double-precision%29) (B :type Float%20%28double-precision%29) (C :type Float%20%28double-precision%29))
  (bind _root (LocalVariables|GetRoot))
  ;[0 0 0] Решение 2 степенного уравнения
  (bind _output_get (LocalVariables|SetD (|((0-((4*A)*C))+(Power(B,2))) A C B)))
  (Utilities|Array|Add _root (|((1/(2*A))*((0-B)-(Sqrt({D6136409-4BDE-8D3C-72A2-D3B2016A083F})))) A B))
  (Utilities|Array|Add _root (|((1/(2*A))*((0-B)+(Sqrt({D6136409-4BDE-8D3C-72A2-D3B2016A083F})))) A B))
  (return (>= _output_get 0.0) (CallFunction|DeleteDublicateRoots _root)))

(fn EducationThirdDegree
  (params (A :type Float%20%28double-precision%29) (B :type Float%20%28double-precision%29) (C :type Float%20%28double-precision%29) (D :type Float%20%28double-precision%29))
  (bind _root (LocalVariables|GetRoot))
  ;[0 0 0] Решение 3 степенного уравнения
  (LocalVariables|SetA1 (/ B A))
  (LocalVariables|SetB1 (/ C A))
  (LocalVariables|SetC1 (/ D A))
  (LocalVariables|SetR (|((((((2*{D1536F54-431B-96C0-69F3-3A946CC20A82})*{D1536F54-431B-96C0-69F3-3A946CC20A82})*{D1536F54-431B-96C0-69F3-3A946CC20A82})-((9*{D1536F54-431B-96C0-69F3-3A946CC20A82})*{D6AC7213-401F-7B4C-2088-71ABD4F3A68F}))+(27*{8A6CEBC6-4037-255E-D60B-F7967C1AC60D}))/54)))
  (LocalVariables|SetQ (|((({D1536F54-431B-96C0-69F3-3A946CC20A82}*{D1536F54-431B-96C0-69F3-3A946CC20A82})-(3*{D6AC7213-401F-7B4C-2088-71ABD4F3A68F}))/9)))
  (bind _output_get (LocalVariables|SetS (|((({A5C957A5-41B3-0261-15B1-4B9AADC0541D}*{A5C957A5-41B3-0261-15B1-4B9AADC0541D})*{A5C957A5-41B3-0261-15B1-4B9AADC0541D})-({F8CB62BB-4EC7-2B19-07F6-63B520ACE598}*{F8CB62BB-4EC7-2B19-07F6-63B520ACE598})))))
  (switch int (CallFunction|SGN _output_get)
    (:-1
      (if (!= (CallFunction|SGN (LocalVariables|GetQ)) 0)
        (LocalVariables|SetCoefficientAngle (|((Abs({F8CB62BB-4EC7-2B19-07F6-63B520ACE598}))/(Sqrt((Power((Abs({A5C957A5-41B3-0261-15B1-4B9AADC0541D})),3)))))))
        (LocalVariables|SetF (|((Loge(((Sqrt(((Power({977B728E-4B3B-7B3C-866F-6C80AE7B761D},2))-X)))+{977B728E-4B3B-7B3C-866F-6C80AE7B761D})))/3) (Math|Conversions|ToFloat(Integer) (CallFunction|SGN (LocalVariables|GetQ)))))
        (Utilities|Array|Add (LocalVariables|GetRoot) (|((((((Power((e(1)),{92E51E72-4DEF-0065-FF11-4494555F9D71}))+((Power((e(1)),(0-{92E51E72-4DEF-0065-FF11-4494555F9D71})))*X))*Y)*(0-1))*(Sqrt((Abs({A5C957A5-41B3-0261-15B1-4B9AADC0541D})))))-({D1536F54-431B-96C0-69F3-3A946CC20A82}/3)) (Math|Conversions|ToFloat(Integer) (CallFunction|SGN (LocalVariables|GetQ))) (Math|Conversions|ToFloat(Integer) (CallFunction|SGN (LocalVariables|GetR)))))
        (else
          (Utilities|Array|Add _root (|((0-(Power(({8A6CEBC6-4037-255E-D60B-F7967C1AC60D}-((Power({D1536F54-431B-96C0-69F3-3A946CC20A82},3))/27)),(1/3))))-({D1536F54-431B-96C0-69F3-3A946CC20A82}/3)))))))
    (:0
      (Utilities|Array|Add _root (|((Power({F8CB62BB-4EC7-2B19-07F6-63B520ACE598},0.333333))-({D1536F54-431B-96C0-69F3-3A946CC20A82}/3)))))
    (:1
      (LocalVariables|SetF (|((Acos(({F8CB62BB-4EC7-2B19-07F6-63B520ACE598}/(Sqrt((Power({A5C957A5-41B3-0261-15B1-4B9AADC0541D},3)))))))/3)))
      (for _index (range -1 1)
        (Utilities|Array|Add (LocalVariables|GetRoot) (|((((Cos(({92E51E72-4DEF-0065-FF11-4494555F9D71}+(((2*PI)/3)/Index))))*(Sqrt({A5C957A5-41B3-0261-15B1-4B9AADC0541D})))*(0-2))-({D1536F54-431B-96C0-69F3-3A946CC20A82}/3)) (Math|Conversions|ToFloat(Integer) _index) (Math|Trig|GetPI))))))
  (return (LocalVariables|GetRoot)))

(fn EducationFourthDegree
  (params (A :type Float%20%28double-precision%29) (B :type Float%20%28double-precision%29) (C :type Float%20%28double-precision%29) (D :type Float%20%28double-precision%29) (E :type Float%20%28double-precision%29))
  (bind _rootseducationseconddegree (LocalVariables|GetRootsEducationSecondDegree))
  ;[0 0 0] Решение 4 степенного уравнения
  (LocalVariables|SetA1 A)
  (LocalVariables|SetB1 B)
  (LocalVariables|SetC1 C)
  (LocalVariables|SetD1 D)
  (LocalVariables|SetE1 E)
  (bind _output_get (LocalVariables|SetR (|((((((256*(Power({781A855D-4B1D-08C9-2D2D-ADAC19D8A025},3)))*{45DFB44A-4FBB-B8D6-2347-52884A1A2940})-((((64*{781A855D-4B1D-08C9-2D2D-ADAC19D8A025})*{781A855D-4B1D-08C9-2D2D-ADAC19D8A025})*{7F726AED-41D9-B448-0FE0-7682F9CBCCEB})*{2FED7B5A-4F48-568B-9DF0-0B97820CCDBD}))+((((16*{781A855D-4B1D-08C9-2D2D-ADAC19D8A025})*{7F726AED-41D9-B448-0FE0-7682F9CBCCEB})*{7F726AED-41D9-B448-0FE0-7682F9CBCCEB})*{96955BF0-46B4-6963-71A6-BB9B467DAFC1}))-(3*(Power({7F726AED-41D9-B448-0FE0-7682F9CBCCEB},4))))/(256*(Power({781A855D-4B1D-08C9-2D2D-ADAC19D8A025},4)))))))
  (bind _output_get_2 (LocalVariables|SetP (|((((8*{781A855D-4B1D-08C9-2D2D-ADAC19D8A025})*{96955BF0-46B4-6963-71A6-BB9B467DAFC1})-((3*{7F726AED-41D9-B448-0FE0-7682F9CBCCEB})*{7F726AED-41D9-B448-0FE0-7682F9CBCCEB}))/((8*{781A855D-4B1D-08C9-2D2D-ADAC19D8A025})*{781A855D-4B1D-08C9-2D2D-ADAC19D8A025})))))
  (LocalVariables|SetQ (|((((((8*{781A855D-4B1D-08C9-2D2D-ADAC19D8A025})*{781A855D-4B1D-08C9-2D2D-ADAC19D8A025})*{2FED7B5A-4F48-568B-9DF0-0B97820CCDBD})-(((4*{781A855D-4B1D-08C9-2D2D-ADAC19D8A025})*{7F726AED-41D9-B448-0FE0-7682F9CBCCEB})*{96955BF0-46B4-6963-71A6-BB9B467DAFC1}))+(({7F726AED-41D9-B448-0FE0-7682F9CBCCEB}*{7F726AED-41D9-B448-0FE0-7682F9CBCCEB})*{7F726AED-41D9-B448-0FE0-7682F9CBCCEB}))/(((8*{781A855D-4B1D-08C9-2D2D-ADAC19D8A025})*{781A855D-4B1D-08C9-2D2D-ADAC19D8A025})*{781A855D-4B1D-08C9-2D2D-ADAC19D8A025}))))
  (bind _output_get_3 (LocalVariables|SetRootsFreeMember (CallFunction|EducationThirdDegree 2.0 (* -1.0 _output_get_2) (* -2.0 _output_get) (|(({1D580F9D-4251-D60C-8273-C6A9EC95582A}*{B8365B89-4EF6-7A0B-C951-D9A0599EE1E0})-(({A6AC6E96-4494-7E00-D29D-8EB53A2A98F7}*{A6AC6E96-4494-7E00-D29D-8EB53A2A98F7})/4))))))
  (bind _array_element (Utilities|Array|ForEachLoopwithBreak _output_get_3 :!label _label)
    (:LoopBody
      (LocalVariables|SetX _array_element)
      (bind _output_get_4 (LocalVariables|SetDifference (|((2*{A814FFF4-4393-8BB2-47A4-4AA1366338DE})-{1D580F9D-4251-D60C-8273-C6A9EC95582A}))))
      (if (> _output_get_4 0.0)
        (LocalVariables|SetPositiveDifference true)
        (goto _label Break)))
    (:Completed
      (if (LocalVariables|GetPositiveDifference)
        (for _index (range 0 1)
          (bind (_exist _roots) (CallFunction|EducationSecondDegree 1.0 (|(Y*(Sqrt({7DCA2E0F-4546-43C2-53E3-83A6989E1E99}))) (Math|Conversions|ToFloat(Integer) (+ _index _index -1))) (|({A814FFF4-4393-8BB2-47A4-4AA1366338DE}-(({A6AC6E96-4494-7E00-D29D-8EB53A2A98F7}/((Sqrt({7DCA2E0F-4546-43C2-53E3-83A6989E1E99}))*2))*Y)) (Math|Conversions|ToFloat(Integer) (+ _index _index -1)))))
          (if _exist
            (Utilities|Array|AppendArray (LocalVariables|GetRootsEducationSecondDegree) _roots)))
        (if (Utilities|Array|IsEmpty _rootseducationseconddegree)
          (return false 0)
          (else
            (for _array_element_2 _rootseducationseconddegree
              (Utilities|Array|Add (LocalVariables|GetRoot) (|(Y-({7F726AED-41D9-B448-0FE0-7682F9CBCCEB}/(4*{781A855D-4B1D-08C9-2D2D-ADAC19D8A025}))) _array_element_2)))
            (return true (CallFunction|DeleteDublicateRoots (LocalVariables|GetRoot)))))
        (else
          (return false 0))))))