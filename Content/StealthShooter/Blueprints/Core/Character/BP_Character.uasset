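; BP_Character is a stealth shooter character handling death and respawn, inventory pickup and interaction detection.
; RebirthDeath toggles mesh ragdoll and collision, moving the capsule with the mesh each tick while dead and returning to LastSavePoint on rebirth.
; ChangeInventory stores added items and updates the UI through the cached BP_GameModeMaze.
; CheckInteractionActor returns the actor hit by a short forward line trace.
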(event `self.ReceiveBeginPlay`
  ;[0 0 0] Сохранение ссылки на гейммод
  (bind _asbp_game_mode_maze (cast `/Game/StealthShooter/Blueprints/Core/GameModes/BP_GameModeMaze` (`GameplayStatics.GetGameMode`)))
  (set `self.GameModeMaze` _asbp_game_mode_maze))

(event `RebirthDeath`
  (params (Rebirth :type Boolean))
  (bind _mesh (`self.Mesh`))
  (bind _brebirth (`self.bRebirth`))
  ;[0 0 0] Смерть и возрождение персонажа
  (bind _output_get (set `self.bRebirth` Rebirth))
  (`PrimitiveComponent.SetCollisionEnabled` (`self.CapsuleComponent`) (select `bool` (`self.bRebirth`) :`false` "NoCollision" :`true` "QueryAndPhysics" :!type "ECollisionEnabled Enum"))
  (set `SceneComponent.bAbsoluteLocation` (not _output_get) (`self.Mesh`))
  (if (`self.bRebirth`)
    (`|ExecutionSequence`
      (:`then_0`
        (`PrimitiveComponent.SetSimulatePhysics` _mesh (not _brebirth) :!label _label))
      (:`then_1`
        (`PrimitiveComponent.SetCollisionEnabled` _mesh (select `bool` _brebirth :`false` "PhysicsOnly" :`true` "NoCollision" :!type "ECollisionEnabled Enum") :!label _label_2))
      (:`then_2`
        (`SceneComponent.K2_SetRelativeTransform` (`self.Mesh`) (`KismetMathLibrary.MakeTransform` (0.0 0.0 -90.0) (struct :`Yaw` -90.0)) false false)
        (`self.K2_SetActorLocation` (`self.LastSavePoint`))))
    (else
      (`|ExecutionSequence`
        (:`then_0`
          (goto _label_2))
        (:`then_1`
          (goto _label))
        (:`then_2`
          (`SceneComponent.K2_SetWorldLocation` (`self.CapsuleComponent`) (+ (`SceneComponent.K2_GetComponentLocation` (`self.Mesh`)) (0.0 0.0 90.0)) false false :!label _label_3)
          (if (not (`self.bRebirth`))
            (`KismetSystemLibrary.DelayUntilNextTick`)
            (goto _label_3)))))))

(event `ChangeInventory`
  (params (Add :type Boolean) (Actor :type "Actor Object Reference (by ref)") (Image :type "Texture2D Object Reference (by ref)"))
  ;[0 0 0] Добавление предмета в инвентарь
  (if Add
    (`BlueprintMapLibrary.Map_Add` (`self.Inventory`) Actor Image)
    (`/Game/StealthShooter/Widgets/WBP_Interface.ChangeInventory` (`/Game/StealthShooter/Blueprints/Core/GameModes/BP_GameModeMaze.Interface` (`self.GameModeMaze`)) true Actor Image)))

(fn `Check Interaction Actor`
  (returns (InteractionActor :type "Actor Object Reference"))
  (bind _scene (`self.Scene`))
  (bind _returnvalue (`SceneComponent.K2_GetComponentLocation` _scene))
  ;[0 0 0] Проверка на наличие интерактивного актора перед персонажем
  (bind _outhit (`KismetSystemLibrary.LineTraceSingle` _returnvalue (+ _returnvalue (* (`SceneComponent.GetForwardVector` _scene) 120.0)) "TraceTypeQuery3"))
  (return (`.HitActor` (`GameplayStatics.BreakHitResult` _outhit))))

(fn `UserConstructionScript`)