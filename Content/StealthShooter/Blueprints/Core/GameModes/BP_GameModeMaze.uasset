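; Game mode for the timed treasure maze, running the flow from main menu through play, pause, respawn and win/defeat screen.
; BeginPlay caches HUD, character and controller, then game instance flags choose menu, fresh restart or save load.
; A looping stopwatch and end timer drive the difficulty-based countdown, and wins update the best time.
; Saving writes player state, inventory and "Save"-tagged actors to one slot, which loading restores.
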(event `self.ReceiveBeginPlay`
  ;[0 0 0] Сохранение нужных ссылок в переменные, запуск или загрузка уровня
  (`|ExecutionSequence`
    (:`then_0`
      (bind _returnvalue (`GameplayStatics.CreateSound2D` "/Game/StealthShooter/Assets/Sound/A_MainMenuMusic.A_MainMenuMusic" 1.0 1.0 0.0 null false false))
      (set `self.MainMenuSound` _returnvalue)
      (bind _returnvalue_2 (`GameplayStatics.CreateSound2D` "/Game/StealthShooter/Assets/Sound/A_MazeMusic.A_MazeMusic" 1.0 1.0 0.0 null false false))
      (set `self.MazeSound` _returnvalue_2))
    (:`then_1`
      (bind _returnvalue_3 (`GameplayStatics.GetActorOfClass` (`self.HUDClass`)))
      (bind _asbp_hudmaze (cast `/Game/StealthShooter/Blueprints/Core/HUD/BP_HUDMaze` _returnvalue_3))
      (set `self.HUD` _asbp_hudmaze))
    (:`then_2`
      (bind _returnvalue_4 (`GameplayStatics.CreateSaveGameObject` "/Game/StealthShooter/Blueprints/Core/BP_SaveMaze.BP_SaveMaze_C"))
      (set `self.SaveGameClass` _returnvalue_4))
    (:`then_3`
      (bind _asbp_character (cast `/Game/StealthShooter/Blueprints/Core/Character/BP_Character` (`GameplayStatics.GetPlayerPawn` 0)))
      (set `self.Character` _asbp_character))
    (:`then_4`
      (bind _asbp_player_controller_maze (cast `/Game/StealthShooter/Blueprints/Core/PlayerController/BP_PlayerControllerMaze` (`GameplayStatics.GetPlayerController` 0)))
      (set `self.PlayerControllerMaze` _asbp_player_controller_maze))
    (:`then_5`
      (bind _asbp_game_instance_maze (cast `/Game/StealthShooter/Blueprints/Core/BP_GameInstanceMaze` (`GameplayStatics.GetGameInstance`)))
      (bind _output_get (set `self.GameInstanceMaze` _asbp_game_instance_maze))
      (if (`/Game/StealthShooter/Blueprints/Core/BP_GameInstanceMaze.Restart` _output_get)
        (set `/Game/StealthShooter/Blueprints/Core/BP_GameInstanceMaze.Restart` false _output_get)
        (`self.StartLevel` true)
        (elif (`/Game/StealthShooter/Blueprints/Core/BP_GameInstanceMaze.Load` _output_get)
          (set `/Game/StealthShooter/Blueprints/Core/BP_GameInstanceMaze.Load` false _output_get)
          (`self.StartLevel` false)
          (else
            (`self.StartGame`)))))))

(event `StartGame`
  (bind _playercontrollermaze (`self.PlayerControllerMaze`))
  (bind _mainmenusound (`self.MainMenuSound`))
  (bind _options_soundvalue (break `/Game/StealthShooter/Blueprints/Structures/Options` (`/Game/StealthShooter/Blueprints/Core/BP_GameInstanceMaze.Options` (`self.GameInstanceMaze`))))
  ;[0 0 0] Начало игры
  (`/Game/StealthShooter/Blueprints/Core/HUD/BP_HUDMaze.ShowWidget` (`self.HUD`) "NewEnumerator1" true "/Game/StealthShooter/Widgets/WBP_MainMenu.WBP_MainMenu_C")
  (`self.DisableInput` _playercontrollermaze _playercontrollermaze)
  (`Controller.SetControlRotation` (`self.PlayerControllerMaze`) (`KismetMathLibrary.ComposeRotators` (`Controller.GetControlRotation` _playercontrollermaze) (struct :`Yaw` 180.0)))
  (`AudioComponent.SetVolumeMultiplier` _mainmenusound _options_soundvalue)
  (`AudioComponent.Play` _mainmenusound 0.0))

(event `Restart`
  ;[0 0 0] Перезапуск уровня
  (set `/Game/StealthShooter/Blueprints/Core/BP_GameInstanceMaze.Restart` true (`self.GameInstanceMaze`))
  (`GameplayStatics.OpenLevel` "Maze"))

(event `StartLevel`
  (params (New :type Boolean))
  (bind _playercontrollermaze (`self.PlayerControllerMaze`))
  ;[0 0 0] Начало уровня
  (set `self.Win` New)
  (`/Game/StealthShooter/Blueprints/Core/HUD/BP_HUDMaze.ShowWidget` (`self.HUD`) "NewEnumerator0" false "/Game/StealthShooter/Widgets/WBP_MainMenu.WBP_MainMenu_C")
  (`self.EnableInput` _playercontrollermaze _playercontrollermaze)
  (bind _outputpin (`/Game/StealthShooter/Blueprints/Core/HUD/BP_HUDMaze.ShowWidget` (`self.HUD`) "NewEnumerator0" true "/Game/StealthShooter/Widgets/WBP_Interface.WBP_Interface_C"))
  (bind _aswbp_interface (cast `/Game/StealthShooter/Widgets/WBP_Interface` _outputpin))
  (set `self.Interface` _aswbp_interface)
  (if (`self.Win`)
    (`self.NewLevel`)
    (else
      (`self.Load`))))

(event `NewLevel`
  (bind _interface (`self.Interface`))
  ;[0 0 0] Начало нового уровня
  (`self.K2_SetActorLocationAndRotation` (`self.Character`) (10100.0 -12769.0 -58.0) (struct :`Yaw` 90.0) false false)
  (`Controller.SetControlRotation` (`self.PlayerControllerMaze`) (`KismetMathLibrary.MakeRotator` 0.0 0.0 90.0))
  (set `self.Time` (select `/Game/StealthShooter/Blueprints/Enums/E_Difficulty` (`/Game/StealthShooter/Blueprints/Core/BP_GameInstanceMaze.Difficulty` (`self.GameInstanceMaze`)) :`NewEnumerator0` 900.0 :`NewEnumerator1` 1200.0 :`NewEnumerator2` 1800.0 :!type "Float (single-precision)"))
  (set `self.Timer` 0.0)
  (`self.ShowTime`)
  (`/Game/StealthShooter/Widgets/WBP_Interface.ShowHealth` (`self.Interface`) 100.0)
  (`KismetSystemLibrary.Delay` 1.0)
  (`/Game/StealthShooter/Widgets/WBP_Interface.ShowMissionText` _interface "Новая миссия!" (make `SlateColor` (struct :`R` 1.0 :`G` 1.0)))
  (`KismetSystemLibrary.Delay` 4.1)
  (`/Game/StealthShooter/Widgets/WBP_Interface.ShowMissionText` _interface "Найти и забрать сокровище в лабиринте" (make `SlateColor` (struct :`R` 1.0 :`G` 1.0 :`B` 1.0))))

(event `ShowTime`
  (bind _mazesound (`self.MazeSound`))
  (bind _options_soundvalue (break `/Game/StealthShooter/Blueprints/Structures/Options` (`/Game/StealthShooter/Blueprints/Core/BP_GameInstanceMaze.Options` (`self.GameInstanceMaze`))))
  ;[0 0 0] Установка секундомера, показ времени, включение музыки
  (`/Game/StealthShooter/Widgets/WBP_Interface.ShowTime` (`self.Interface`) (`self.Time`))
  (bind _returnvalue (`KismetSystemLibrary.K2_SetTimerDelegate` (delegate `Stopwatch`) 1.0 true))
  (set `self.TimerStopwwatch` _returnvalue)
  (bind _returnvalue_2 (`KismetSystemLibrary.K2_SetTimerDelegate` (delegate `EndGameTimer`) (`self.Time`)))
  (set `self.TimerEndGame` _returnvalue_2)
  (bind _mainmenusound (`self.MainMenuSound`)
    (:`then`
      (`AudioComponent.Stop` _mainmenusound))
    (:`else`
      _))
  (`AudioComponent.SetVolumeMultiplier` _mazesound _options_soundvalue)
  (`AudioComponent.Play` _mazesound 0.0))

(event `Stopwatch`
  ;[0 0 0] Установка секундомера, показ времени, включение музыки
  (bind _output_get (set `self.Time` (- (`self.Time`) 1.0)))
  (`/Game/StealthShooter/Widgets/WBP_Interface.ShowTime` (`self.Interface`) _output_get)
  (set `self.Timer` (+ (`self.Timer`) 1.0)))

(event `EndGameTimer`
  ;[0 0 0] Установка секундомера, показ времени, включение музыки
  (`KismetSystemLibrary.K2_ClearAndInvalidateTimerHandle` (`self.TimerStopwwatch`))
  (`KismetSystemLibrary.K2_ClearAndInvalidateTimerHandle` (`self.TimerEndGame`))
  (`self.EndGame` false))

(event `Load`
  (bind _character (`self.Character`))
  (bind _interface (`self.Interface`))
  (bind _gameinstancemaze (`self.GameInstanceMaze`))
  (bind _savegameclass (`self.SaveGameClass`))
  (bind _locationsmagiccubes (`/Game/StealthShooter/Blueprints/Core/BP_SaveMaze.LocationsMagicCubes` _savegameclass))
  (bind _inventory (`/Game/StealthShooter/Blueprints/Core/BP_SaveMaze.Inventory` (`self.SaveGameClass`)))
  (bind _bp_health (`/Game/StealthShooter/Blueprints/Core/Character/BP_Character.BP_Health` _character))
  ;[0 0 0] Загрузка уровня
  (bind _returnvalue (`GameplayStatics.LoadGameFromSlot` "FirstSlot"))
  (bind _asbp_save_maze (cast `/Game/StealthShooter/Blueprints/Core/BP_SaveMaze` _returnvalue)
    (:`then`
      (bind _output_get (set `self.SaveGameClass` _asbp_save_maze))
      (set `/Game/StealthShooter/Blueprints/Core/BP_GameInstanceMaze.Rating` (`/Game/StealthShooter/Blueprints/Core/BP_SaveMaze.Rating` _output_get) _gameinstancemaze)
      (set `/Game/StealthShooter/Blueprints/Core/BP_GameInstanceMaze.Options` (`/Game/StealthShooter/Blueprints/Core/BP_SaveMaze.Options` _savegameclass) _gameinstancemaze)
      (set `/Game/StealthShooter/Blueprints/Core/BP_GameInstanceMaze.Difficulty` (`/Game/StealthShooter/Blueprints/Core/BP_SaveMaze.Difficulty` _savegameclass) _gameinstancemaze)
      (set `self.Time` (`/Game/StealthShooter/Blueprints/Core/BP_SaveMaze.Time` _savegameclass))
      (set `self.Timer` (`/Game/StealthShooter/Blueprints/Core/BP_SaveMaze.Timer` _savegameclass))
      (set `/Game/StealthShooter/Blueprints/Core/Character/BP_Character.Keys` (`/Game/StealthShooter/Blueprints/Core/BP_SaveMaze.Keys` _savegameclass) _character)
      (set `/Game/StealthShooter/Blueprints/Core/Character/BP_Character.bTreasure` (`/Game/StealthShooter/Blueprints/Core/BP_SaveMaze.Treasure` _savegameclass) _character)
      (set `/Game/StealthShooter/Blueprints/Core/Character/BP_Character.bBoots` (`/Game/StealthShooter/Blueprints/Core/BP_SaveMaze.Boots` _savegameclass) _character)
      (set `/Game/StealthShooter/Blueprints/Core/Character/BP_Character.LastSavePoint` (`/Game/StealthShooter/Blueprints/Core/BP_SaveMaze.SavePointPlayer` _savegameclass) _character)
      (`self.K2_SetActorTransform` _character (`/Game/StealthShooter/Blueprints/Core/BP_SaveMaze.PlayerTransform` _savegameclass) false false)
      (bind _output_get_2 (set `/Game/StealthShooter/Blueprints/Components/BP_Health.Health` (`/Game/StealthShooter/Blueprints/Core/BP_SaveMaze.Health` _savegameclass) _bp_health))
      (`/Game/StealthShooter/Widgets/WBP_Interface.ShowHealth` _interface _output_get_2)
      (bind _output_get_3 (set `/Game/StealthShooter/Blueprints/Components/BP_Health.Deaths` (`/Game/StealthShooter/Blueprints/Core/BP_SaveMaze.Deaths` _savegameclass) _bp_health))
      (`/Game/StealthShooter/Widgets/WBP_Interface.ShowDeaths` _interface _output_get_3)
      (for _array_element _locationsmagiccubes
        (`/Engine/EditorBlueprintResources/StandardMacros.IsValid` (break `/Game/StealthShooter/Blueprints/Structures/SaveActors` _array_element)
          (:`Is Valid`
            (`self.K2_SetActorTransform` (break `/Game/StealthShooter/Blueprints/Structures/SaveActors` _array_element) (`.Transform_15_A4E11C02479610B9740E1AA75C3440A1` (break `/Game/StealthShooter/Blueprints/Structures/SaveActors` _array_element)) false true)
            (`self.SetActorHiddenInGame` (break `/Game/StealthShooter/Blueprints/Structures/SaveActors` _array_element) (`.Hidden_8_40FF9B8544FF355F7D461490DC99CD48` (break `/Game/StealthShooter/Blueprints/Structures/SaveActors` _array_element)))
            (`self.SetActorEnableCollision` (break `/Game/StealthShooter/Blueprints/Structures/SaveActors` _array_element) (`.Collision_13_C208DA5840E939E9D7774990C78A82DD` (break `/Game/StealthShooter/Blueprints/Structures/SaveActors` _array_element)))
            (if (!= (`KismetArrayLibrary.Array_Find` (`.Tags_19_5DFC321E4098C70D5E99CEB1E6772056` (break `/Game/StealthShooter/Blueprints/Structures/SaveActors` _array_element)) "Active") -1)
              (message `/Game/StealthShooter/Blueprints/Interface/BPI_SaveGame.LoadGame` (break `/Game/StealthShooter/Blueprints/Structures/SaveActors` _array_element))))))
      (`KismetArrayLibrary.Array_Clear` _locationsmagiccubes)
      (`self.ShowTime`)
      (`KismetSystemLibrary.DelayUntilNextTick`)
      (bind _keys (`BlueprintMapLibrary.Map_Keys` _inventory))
      (for _array_element_2 _keys
        (`/Game/StealthShooter/Blueprints/Core/Character/BP_Character.ChangeInventory` (`self.Character`) true _array_element_2 (`BlueprintMapLibrary.Map_Find` _inventory _array_element_2))))
    (:`CastFailed`
      (`self.NewLevel`))))

(event `SaveGame`
  (bind _savegameclass (`self.SaveGameClass`))
  (bind _character (`self.Character`))
  (bind _character_2 (`self.Character`))
  (bind _gameinstancemaze (`self.GameInstanceMaze`))
  (bind _bp_health (`/Game/StealthShooter/Blueprints/Core/Character/BP_Character.BP_Health` _character))
  ;[0 0 0] Сохранение игры
  (set `/Game/StealthShooter/Blueprints/Core/BP_SaveMaze.Timer` (`self.Timer`) _savegameclass)
  (set `/Game/StealthShooter/Blueprints/Core/BP_SaveMaze.Time` (`self.Time`) _savegameclass)
  (set `/Game/StealthShooter/Blueprints/Core/BP_SaveMaze.Keys` (`/Game/StealthShooter/Blueprints/Core/Character/BP_Character.Keys` _character) _savegameclass)
  (set `/Game/StealthShooter/Blueprints/Core/BP_SaveMaze.Health` (`/Game/StealthShooter/Blueprints/Components/BP_Health.Health` _bp_health) _savegameclass)
  (set `/Game/StealthShooter/Blueprints/Core/BP_SaveMaze.Deaths` (`/Game/StealthShooter/Blueprints/Components/BP_Health.Deaths` _bp_health) _savegameclass)
  (set `/Game/StealthShooter/Blueprints/Core/BP_SaveMaze.Boots` (`/Game/StealthShooter/Blueprints/Core/Character/BP_Character.bBoots` _character) _savegameclass)
  (set `/Game/StealthShooter/Blueprints/Core/BP_SaveMaze.Treasure` (`/Game/StealthShooter/Blueprints/Core/Character/BP_Character.bTreasure` _character) _savegameclass)
  (set `/Game/StealthShooter/Blueprints/Core/BP_SaveMaze.PlayerTransform` (`self.GetTransform` _character_2) _savegameclass)
  (set `/Game/StealthShooter/Blueprints/Core/BP_SaveMaze.SavePointPlayer` (`/Game/StealthShooter/Blueprints/Core/Character/BP_Character.LastSavePoint` _character_2) _savegameclass)
  (set `/Game/StealthShooter/Blueprints/Core/BP_SaveMaze.Options` (`/Game/StealthShooter/Blueprints/Core/BP_GameInstanceMaze.Options` _gameinstancemaze) _savegameclass)
  (set `/Game/StealthShooter/Blueprints/Core/BP_SaveMaze.Rating` (`/Game/StealthShooter/Blueprints/Core/BP_GameInstanceMaze.Rating` _gameinstancemaze) _savegameclass)
  (set `/Game/StealthShooter/Blueprints/Core/BP_SaveMaze.Difficulty` (`/Game/StealthShooter/Blueprints/Core/BP_GameInstanceMaze.Difficulty` _gameinstancemaze) _savegameclass)
  (set `/Game/StealthShooter/Blueprints/Core/BP_SaveMaze.Inventory` (`/Game/StealthShooter/Blueprints/Core/Character/BP_Character.Inventory` (`self.Character`)) _savegameclass)
  (bind _outactors (`GameplayStatics.GetAllActorsWithTag` "Save"))
  (for _array_element _outactors
    (`KismetArrayLibrary.Array_Add` (`/Game/StealthShooter/Blueprints/Core/BP_SaveMaze.LocationsMagicCubes` (`self.SaveGameClass`)) (make `/Game/StealthShooter/Blueprints/Structures/SaveActors` _array_element (`self.GetTransform` _array_element) (`Actor.bHidden` _array_element) (`self.GetActorEnableCollision` _array_element) (`Actor.Tags` _array_element))))
  (`GameplayStatics.SaveGameToSlot` (`self.SaveGameClass`) "FirstSlot"))

(event `RebirthPlayer`
  (bind _playercontrollermaze (`self.PlayerControllerMaze`))
  (bind _playercontrollermaze_2 (`self.PlayerControllerMaze`))
  (bind _character (`self.Character`))
  ;[0 0 0] Возрождение персонажа
  (`/Game/StealthShooter/Blueprints/Core/Character/BP_Character.RebirthDeath` _character false)
  (`self.DisableInput` _playercontrollermaze _playercontrollermaze)
  (`KismetSystemLibrary.Delay` 2.0)
  (`/Game/StealthShooter/Blueprints/Core/Character/BP_Character.RebirthDeath` _character true)
  (`self.OnRebirthPlayer`)
  (`self.EnableInput` _playercontrollermaze_2 _playercontrollermaze_2))

(event `EndGame`
  (params (Win :type Boolean))
  (bind _win (`self.Win`))
  ;[0 0 0] Конец игры, остановка таймеров, перезаписывание рекорда, показ виджета конца игры
  (set `self.Win` Win)
  (`KismetSystemLibrary.K2_ClearAndInvalidateTimerHandle` (`self.TimerEndGame`))
  (`KismetSystemLibrary.K2_ClearAndInvalidateTimerHandle` (`self.TimerStopwwatch`))
  (if (`self.Win`)
    (bind _structout (setmembers `/Game/StealthShooter/Blueprints/Structures/Rating` :`StructRef` (`/Game/StealthShooter/Blueprints/Core/BP_GameInstanceMaze.Rating` (`self.GameInstanceMaze`)) :`Deaths` (`/Game/StealthShooter/Blueprints/Components/BP_Health.Deaths` (`/Game/StealthShooter/Blueprints/Core/Character/BP_Character.BP_Health` (`self.Character`))) :`Time` (`self.Timer`)))
    (if (or (== (break `/Game/StealthShooter/Blueprints/Structures/Rating` _structout) 0.0) (< (`self.Timer`) (break `/Game/StealthShooter/Blueprints/Structures/Rating` _structout)))
      (setmembers `/Game/StealthShooter/Blueprints/Structures/Rating` :`StructRef` (`/Game/StealthShooter/Blueprints/Core/BP_GameInstanceMaze.Rating` (`self.GameInstanceMaze`)) :`BestTime` (`self.Timer`))))
  (bind _outputpin (`/Game/StealthShooter/Blueprints/Core/HUD/BP_HUDMaze.ShowWidget` (`self.HUD`) "NewEnumerator1" true "/Game/StealthShooter/Widgets/WBP_EndGame.WBP_EndGame_C"))
  (bind _aswbp_end_game (cast `/Game/StealthShooter/Widgets/WBP_EndGame` _outputpin))
  (`/Game/StealthShooter/Widgets/WBP_EndGame.EndGame` _aswbp_end_game _win)
  (`AudioComponent.Stop` (`self.MazeSound`))
  (`GameplayStatics.PlaySound2D` (select `bool` _win :`false` "/Game/StealthShooter/Assets/Sound/A_Defeat.A_Defeat" :`true` "/Game/StealthShooter/Assets/Sound/A_Win.A_Win" :!type "SoundBase Object Reference") 1.0 1.0 0.0 null null))

(event `QuitGame`
  ;[0 0 0] Выход из игры
  (set `/Game/StealthShooter/Blueprints/Core/BP_GameInstanceMaze.Rating` (`/Game/StealthShooter/Blueprints/Core/BP_SaveMaze.Rating` (`self.SaveGameClass`)) (`self.GameInstanceMaze`))
  (`KismetSystemLibrary.QuitGame` null "Quit"))

(event `PauseGame`
  (bind _returnvalue (`GameplayStatics.IsGamePaused`))
  ;[0 0 0] Пауза в игре
  (`GameplayStatics.SetGamePaused` (not _returnvalue))
  (`/Game/StealthShooter/Blueprints/Core/HUD/BP_HUDMaze.ShowWidget` (`self.HUD`) (select `bool` _returnvalue :`false` "NewEnumerator0" :`true` "NewEnumerator2" :!type "/Game/StealthShooter/Blueprints/Enums/E_InputGame Enum") _returnvalue "/Game/StealthShooter/Widgets/WBP_PauseMenu.WBP_PauseMenu_C"))

(fn `UserConstructionScript`)