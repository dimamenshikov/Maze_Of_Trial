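; Player controller for the maze mode, routing Enhanced Input to the character, game mode and event dispatchers.
; BeginPlay adds the maze mapping context and caches game mode and character for movement, look, jump, interaction and pause.
; A MappingInput switch makes Move either walk the pawn or broadcast plate selection for the tag-game puzzle.
; Plate shifting and inventory actions also broadcast, while holding super jump with boots temporarily raises jump velocity.
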(event `self.ReceiveBeginPlay`
  ;[0 0 0] Сохранение нужных ссылок в переменные
  (`|ExecutionSequence`
    (:`then_0`
      (`EnhancedInputSubsystemInterface.AddMappingContext` (subsystem `EnhancedInputLocalPlayerSubsystem`) "/Game/StealthShooter/Blueprints/Input/IMC_Maze.IMC_Maze" 0 (struct)))
    (:`then_1`
      (bind _asbp_game_mode_maze (cast `/Game/StealthShooter/Blueprints/Core/GameModes/BP_GameModeMaze` (`GameplayStatics.GetGameMode`)))
      (set `self.GameModeMaze` _asbp_game_mode_maze))
    (:`then_2`
      (bind _asbp_character (cast `/Game/StealthShooter/Blueprints/Core/Character/BP_Character` (`GameplayStatics.GetPlayerPawn` 0)))
      (set `self.Person` _asbp_character))))

(event `EnhancedInput|/Game/StealthShooter/Blueprints/Input/Actions/AI_Move`
  (params (ActionValue :type "Vector2D Structure") (ElapsedSeconds :type "Float (double-precision)") (TriggeredSeconds :type "Float (double-precision)") (InputAction :type "InputAction Object Reference" :default "/Game/StealthShooter/Blueprints/Input/Actions/AI_Move.AI_Move"))
  (bind (_returnvalue_roll _returnvalue_pitch _returnvalue_yaw) (`KismetMathLibrary.BreakRotator` (`self.GetControlRotation`)))
  (bind _mappinginput (`self.MappingInput`))
  ;[0 0 0] Движение персонажа или выборка плит
  (:`Triggered`
    (switch `/Game/StealthShooter/Blueprints/Enums/E_MappingInput` _mappinginput
      (:`NewEnumerator0`
        (`Pawn.AddMovementInput` (`GameplayStatics.GetPlayerPawn` 0) (`KismetMathLibrary.GreaterGreater_VectorRotator` (`KismetMathLibrary.Conv_Vector2DToVector` ActionValue) (`KismetMathLibrary.MakeRotator` 0.0 0.0 _returnvalue_yaw)) 1.0 false))))
  (:`Started`
    (switch `/Game/StealthShooter/Blueprints/Enums/E_MappingInput` _mappinginput
      (:`NewEnumerator1`
        (`self.OnBlick` ActionValue)))))

(event `EnhancedInput|/Game/StealthShooter/Blueprints/Input/Actions/AI_Look`
  (params (ActionValue :type "Vector2D Structure") (ElapsedSeconds :type "Float (double-precision)") (TriggeredSeconds :type "Float (double-precision)") (InputAction :type "InputAction Object Reference" :default "/Game/StealthShooter/Blueprints/Input/Actions/AI_Look.AI_Look"))
  ;[0 0 0] Вращение камерой
  (:`Triggered`
    (`self.AddYawInput` ActionValue_X)
    (`self.AddPitchInput` ActionValue_Y)))

(event `EnhancedInput|/Game/StealthShooter/Blueprints/Input/Actions/AI_Jump`
  (params (ActionValue :type Boolean) (ElapsedSeconds :type "Float (double-precision)") (TriggeredSeconds :type "Float (double-precision)") (InputAction :type "InputAction Object Reference" :default "/Game/StealthShooter/Blueprints/Input/Actions/AI_Jump.AI_Jump"))
  ;[0 0 0] Прыжок
  (:`Started`
    (bind _person (`self.Person`)
      (:`then`
        (`Character.Jump` _person)
        (bind _charactermovement (`Character.CharacterMovement` _person))
        (if (and (== (`CharacterMovementComponent.JumpZVelocity` _charactermovement) 1500.0) (not (`NavMovementComponent.IsFalling` _charactermovement)))
          (`GameplayStatics.SpawnSound2D` "/Game/StealthShooter/Assets/Sound/A_Jump.A_Jump" 1.0 1.0 10.0 null)))
      (:`else`))))

(event `EnhancedInput|/Game/StealthShooter/Blueprints/Input/Actions/AI_PlateOffset`
  (params (ActionValue :type Boolean) (ElapsedSeconds :type "Float (double-precision)") (TriggeredSeconds :type "Float (double-precision)") (InputAction :type "InputAction Object Reference" :default "/Game/StealthShooter/Blueprints/Input/Actions/AI_PlateOffset.AI_PlateOffset"))
  ;[0 0 0] Перемещение плит
  (:`Started`
    (`self.OnOffsetPlate`)))

(event `EnhancedInput|/Game/StealthShooter/Blueprints/Input/Actions/AI_Interaction`
  (params (ActionValue :type Boolean) (ElapsedSeconds :type "Float (double-precision)") (TriggeredSeconds :type "Float (double-precision)") (InputAction :type "InputAction Object Reference" :default "/Game/StealthShooter/Blueprints/Input/Actions/AI_Interaction.AI_Interaction"))
  ;[0 0 0] Проверка и взаимодействие с предметом
  (:`Started`
    (bind _interactionactor (`/Game/StealthShooter/Blueprints/Core/Character/BP_Character.Check Interaction Actor` (`self.Person`)))
    (message `/Game/StealthShooter/Blueprints/Interface/BPI_Interaction.Interaction` _interactionactor true)))

(event `EnhancedInput|/Game/StealthShooter/Blueprints/Input/Actions/AI_Pause`
  (params (ActionValue :type Boolean) (ElapsedSeconds :type "Float (double-precision)") (TriggeredSeconds :type "Float (double-precision)") (InputAction :type "InputAction Object Reference" :default "/Game/StealthShooter/Blueprints/Input/Actions/AI_Pause.AI_Pause"))
  ;[0 0 0] Пауза
  (:`Started`
    (`/Game/StealthShooter/Blueprints/Core/GameModes/BP_GameModeMaze.PauseGame` (`self.GameModeMaze`))))

(event `EnhancedInput|/Game/StealthShooter/Blueprints/Input/Actions/AI_ActivateSuperJump`
  (params (ActionValue :type Boolean) (ElapsedSeconds :type "Float (double-precision)") (TriggeredSeconds :type "Float (double-precision)") (InputAction :type "InputAction Object Reference" :default "/Game/StealthShooter/Blueprints/Input/Actions/AI_ActivateSuperJump.AI_ActivateSuperJump"))
  (bind _person (`self.Person`))
  (bind _bboots (`/Game/StealthShooter/Blueprints/Core/Character/BP_Character.bBoots` _person))
  (bind _charactermovement (`Character.CharacterMovement` _person))
  ;[0 0 0] Увеличение прыжка
  (:`Started`
    (if _bboots
      (set `CharacterMovementComponent.JumpZVelocity` 1500.0 _charactermovement)))
  (:`Completed`
    (if _bboots
      (set `CharacterMovementComponent.JumpZVelocity` 500.0 _charactermovement))))

(event `EnhancedInput|/Game/StealthShooter/Blueprints/Input/Actions/AI_Inventory`
  (params (ActionValue :type Boolean) (ElapsedSeconds :type "Float (double-precision)") (TriggeredSeconds :type "Float (double-precision)") (InputAction :type "InputAction Object Reference" :default "/Game/StealthShooter/Blueprints/Input/Actions/AI_Inventory.AI_Inventory"))
  ;[0 0 0] Показ и сокрытие инвентаря и управления
  (:`Started`
    (`self.OnInventory` true))
  (:`Completed`
    (`self.OnInventory` false)))

(event `EnhancedInput|/Game/StealthShooter/Blueprints/Input/Actions/AI_Scroll`
  (params (ActionValue :type "Float (double-precision)") (ElapsedSeconds :type "Float (double-precision)") (TriggeredSeconds :type "Float (double-precision)") (InputAction :type "InputAction Object Reference" :default "/Game/StealthShooter/Blueprints/Input/Actions/AI_Scroll.AI_Scroll"))
  ;[0 0 0] Прокрутка инвентаря
  (:`Triggered`
    (`self.OnScroll` ActionValue)))

(fn `UserConstructionScript`)